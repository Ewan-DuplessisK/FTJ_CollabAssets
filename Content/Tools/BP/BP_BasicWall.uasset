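; BP_BasicWall is a Geometry Script tool actor that procedurally builds a wall with a cutout.
; On rebuild it appends a box and boolean-subtracts an extruded rectangle, optionally rounded, remapped to a separate material slot.
; It then optionally bevels by angle-derived polygroups, assigns wall and cutout materials, and recomputes scaled UVs.
; Two custom events bake the dynamic mesh to a new static mesh asset or update the stored one, copying materials across.
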(event `self.OnRebuildGeneratedMesh`
  (params (TargetMesh :type "DynamicMesh Object Reference"))
  (bind (_wallsize_x _wallsize_y _wallsize_z) (`KismetMathLibrary.BreakVector` (`self.WallSize`)))
  (bind (_cutoutsize_x _cutoutsize_y _cutoutsize_z) (`KismetMathLibrary.BreakVector` (`self.CutoutSize`)))
  (bind (_cutoutsize_x_2 _cutoutsize_y_2) (`KismetMathLibrary.BreakVector` (`self.CutoutSize`)))
  (bind (_cutoutsize_x_3 _cutoutsize_y_3 _cutoutsize_z_2) (`KismetMathLibrary.BreakVector` (`self.CutoutSize`)))
  (set `self.DynamicMesh` TargetMesh)
  (`|ExecutionSequence`
    (:`then_0`
      ; Create Wall
      (`GeometryScriptLibrary_MeshPrimitiveFunctions.AppendBox` (`self.DynamicMesh`) (struct) (struct) _wallsize_x _wallsize_y _wallsize_z 0 0 0 "Base" null))
    (:`then_1`
      (if (`self.IsCutoutRounded?`)
        ; Create Rounded Cutout
        (bind _returnvalue (`self.AllocateComputeMesh`))
        (bind _returnvalue_2 (`GeometryScriptLibrary_MeshPrimitiveFunctions.AppendRoundRectangleXY` _returnvalue (struct) (`KismetMathLibrary.MakeTransform` (0.0 0.0 0.0) (struct :`Roll` 90.0)) _cutoutsize_x _cutoutsize_z (`self.Corner Radius`) 0 0 (`self.Steps Round`) null))
        (set `self.CutoutMesh` _returnvalue_2)
        (else
          ; Create Cutout
          (bind _returnvalue_3 (`self.AllocateComputeMesh`))
          (bind _returnvalue_4 (`GeometryScriptLibrary_MeshPrimitiveFunctions.AppendRectangleXY` _returnvalue_3 (struct) (`KismetMathLibrary.MakeTransform` (0.0 0.0 0.0) (struct :`Roll` 90.0)) _cutoutsize_x_3 _cutoutsize_z_2 0 0 null))
          (set `self.CutoutMesh` _returnvalue_4))))
    (:`then_2`
      ; Extrude Cutout
      (bind _returnvalue_5 (`GeometryScriptLibrary_MeshModelingFunctions.ApplyMeshExtrude_Compatibility_5p0` (`self.CutoutMesh`) (make `GeometryScriptMeshExtrudeOptions` _cutoutsize_y_2 (0.0 1.0 0.0)) null))
      (bind _returnvalue_6 (`GeometryScriptLibrary_MeshMaterialFunctions.RemapMaterialIDs` _returnvalue_5 0 1 null))
      (set `self.CutoutMesh` _returnvalue_6))
    (:`then_3`
      ; Apply Cutout Boolean
      (bind _returnvalue_7 (`GeometryScriptLibrary_MeshBooleanFunctions.ApplyMeshBoolean` (`self.DynamicMesh`) (struct) (`self.CutoutMesh`) (`self.CutoutTransform`) "Subtract" (struct) null))
      (set `self.DynamicMesh` _returnvalue_7))
    (:`then_4`
      ; Do Bevels
      (if (`self.IsBeveled?`)
        (bind _returnvalue_8 (`GeometryScriptLibrary_MeshPolygroupFunctions.ComputePolygroupsFromAngleThreshold` (`self.DynamicMesh`) (struct) 25.0 2 null))
        (bind _returnvalue_9 (`GeometryScriptLibrary_MeshModelingFunctions.ApplyMeshPolygroupBevel` _returnvalue_8 (make `GeometryScriptMeshBevelOptions` (`self.BevelAmount`)) null))
        (bind _returnvalue_10 (`GeometryScriptLibrary_MeshNormalsFunctions.ComputeSplitNormals` _returnvalue_9 (make `GeometryScriptSplitNormalsOptions` true 25.0) (struct) null))
        (set `self.DynamicMesh` _returnvalue_10)))
    (:`then_5`
      ; Setup Materials
      (`DynamicMeshComponent.ConfigureMaterialSet` (`self.DynamicMeshComponent`) (`|MakeArray` (`self.WallMaterial`) (`self.CutoutMaterial`)) true))
    (:`then_6`
      ; Recompute and Scale UVs
      (bind _returnvalue_11 (`GeometryScriptLibrary_MeshUVFunctions.RecomputeMeshUVs` (`self.DynamicMesh`) 0 (struct) (struct) null))
      (`GeometryScriptLibrary_MeshUVFunctions.ScaleMeshUVs` _returnvalue_11 0 (`KismetMathLibrary.MakeVector2D` (`self.UVScaleX`) (`self.UVScaleY`)) (0.0 0.0) (struct) null))))

(event `CustomEvent`
  ; Generate New Static Mesh
  (bind _returnvalue (`BaseDynamicMeshComponent.GetDynamicMesh` (`self.DynamicMeshComponent`)))
  (bind _uniqueassetpathandname (`GeometryScriptLibrary_CreateNewAssetFunctions.CreateUniqueNewAssetPathName` (`self.Asset Folder Path`) (`KismetSystemLibrary.GetDisplayName` self) (struct) null)
    (:`Success`
      (bind _returnvalue_2 (`GeometryScriptLibrary_CreateNewAssetFunctions.CreateNewStaticMeshAssetFromMesh` _returnvalue _uniqueassetpathandname (make `GeometryScriptCreateNewStaticMeshAssetOptions` false false false (struct :`bLerpUVs` true :`bVoxelNDF` true :`PositionPrecision` -2147483648 :`NormalPrecision` -1 :`TangentPrecision` -1 :`BoneWeightPrecision` -1 :`KeepPercentTriangles` 1.0 :`GenerateFallback` "PlatformDefault" :`FallbackTarget` "Auto" :`FallbackPercentTriangles` 1.0 :`FallbackRelativeError` 1.0 :`NumRays` 1 :`NaniteAssemblyData` (struct)) 0.0 true "CTF_UseComplexAsSimple") null)
        (:`Success`
          (bind _output_get (set `self.Static Mesh Asset` _returnvalue_2))
          (for (_array_element _array_index) (`MeshComponent.GetMaterials` (`self.DynamicMeshComponent`))
            (`StaticMesh.SetMaterial` _output_get _array_index _array_element)))))))

(event `CustomEvent_1`
  ; Update Static Mesh
  (bind _returnvalue (`BaseDynamicMeshComponent.GetDynamicMesh` (`self.DynamicMeshComponent`)))
  (`GeometryScriptLibrary_StaticMeshFunctions.CopyMeshToStaticMesh` _returnvalue (`self.Static Mesh Asset`) (struct) (struct) true null
    (:`Success`
      (for (_array_element _array_index) (`MeshComponent.GetMaterials` (`self.DynamicMeshComponent`))
        (`StaticMesh.SetMaterial` (`self.Static Mesh Asset`) _array_index _array_element)))))

(fn `UserConstructionScript`
  (`parent.UserConstructionScript`))