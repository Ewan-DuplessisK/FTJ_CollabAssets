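; Charger enemy that patrols along a spline until it sees a pawn, then turns toward the player and charges in a straight line.
; Looping timers drive tracking and swept movement to a sphere-traced target, with tuning read from a data asset.
; Charge hits damage and knock back the player; charge endings and obstacle impacts stun it, then tracking resumes.
; Kicks launch and damage it; other hits hurt only from the front, except AOE props.
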(event `self.ReceiveBeginPlay`
  (`self.ResumePatrol`)
  (set `self.MaxHealth` (`/Game/Characters/Enemies/PDA_ChargerEnemy.Max Health` (`self.DataAsset`))))

(event `self.ReceiveTick`
  (params (DeltaSeconds :type "Float (single-precision)")))

(event `self.PawnSensing.OnSeePawn`
  (params (Pawn :type "Pawn Object Reference"))
  (`KismetSystemLibrary.K2_ClearAndInvalidateTimerHandle` (`self.PatrolHandle`))
  (`MovementComponent.StopMovementImmediately` (`self.CharacterMovement`))
  (`Controller.StopMovement` (`AIBlueprintHelperLibrary.GetAIController` self))
  (`/Engine/EditorBlueprintResources/StandardMacros.DoOnce` false :!label _label
    (:`Completed`
      (`self.PrepareCharge`))))

(event `ResetCharge`
  (goto _label :!via `Reset`))

(event `self.ReceiveHit`
  (params (MyComp :type "PrimitiveComponent Object Reference") (Other :type "Actor Object Reference") (OtherComp :type "PrimitiveComponent Object Reference") (bSelfMoved :type Boolean) (HitLocation :type "Vector Structure") (HitNormal :type "Vector Structure") (NormalImpulse :type "Vector Structure") (Hit :type "HitResult Structure (by ref)"))
  (bind _returnvalue (`PrimitiveComponent.GetCollisionObjectType` OtherComp))
  (if (`self.IsCharging`)
    (if (`self.ActorHasTag` Other "Player")
      (message `HitInterface.GetHit` Other (`/Game/Characters/Enemies/PDA_ChargerEnemy.Damage` (`self.DataAsset`)) 0.0 (* (`self.GetActorForwardVector`) (`/Game/Characters/Enemies/PDA_ChargerEnemy.PushMultiplier` (`self.DataAsset`))) 0.0 self)
      (`self.InterruptCharge`)
      (else
        (switch `ECollisionChannel` _returnvalue
          (:`ECC_WorldStatic`
            (`self.Stun` (`/Game/Characters/Enemies/PDA_ChargerEnemy.WallStunDuration` (`self.DataAsset`)) true :!label _label_2))
          (:`ECC_GameTraceChannel6`
            (`self.Stun` (`/Game/Characters/Enemies/PDA_ChargerEnemy.BasicStunDuration` (`self.DataAsset`))))
          (:`ECC_GameTraceChannel11`
            (goto _label_2)))))
    (elif (`self.IsKicked`)
      (switch `ECollisionChannel` _returnvalue
        (:`ECC_WorldStatic`
          (goto _label_2))
        (:`ECC_GameTraceChannel11`
          (goto _label_2))))))

(event `KickedInterface.Kicked`
  (params (KickVector :type "Vector Structure") (PlayerPosition :type "Vector Structure"))
  (`KismetSystemLibrary.K2_ClearAndInvalidateTimerHandle` (`self.PatrolHandle`))
  (`PrimitiveComponent.AddImpulse` (`self.CapsuleComponent`) (* KickVector (`/Game/Characters/Enemies/PDA_ChargerEnemy.KickForceMultiplier` (`self.DataAsset`))) "None" true)
  (set `self.IsKicked` true)
  (`HealthInterface.RemoveHealth` (`/Game/Characters/Enemies/PDA_ChargerEnemy.DamageFromKick` (`self.DataAsset`))))

(event `Stun`
  (params (Duration :type "Float (double-precision)") (IsWallStun :type Boolean))
  (if IsWallStun
    (`KismetSystemLibrary.K2_ClearAndInvalidateTimerHandle` (`self.StunHandle`))
    (set `self.IsStunned` true :!label _label_3)
    (bind _returnvalue (`KismetSystemLibrary.K2_SetTimer` null "ResetStun" Duration))
    (set `self.StunHandle` _returnvalue)
    (elif (not (`KismetSystemLibrary.K2_IsValidTimerHandle` (`self.StunHandle`)))
      (goto _label_3))))

(event `HitInterface.GetHit`
  (params (Damage :type "Float (single-precision)") (HitStunDuration :type "Float (single-precision)") (KnockbackVector :type "Vector Structure") (InvincibilityTime :type "Float (single-precision)") (SourceActor :type "Actor Object Reference"))
  (`KismetSystemLibrary.K2_ClearAndInvalidateTimerHandle` (`self.PatrolHandle`))
  (`/Engine/EditorBlueprintResources/StandardMacros.IsValid` SourceActor
    (:`Is Valid`
      (cast `/Game/BPs/VacuumProps/BP_SuckableProp_AOE` SourceActor
        (:`then`
          (`HealthInterface.RemoveHealth` Damage :!label _label_4))
        (:`CastFailed`
          (if (< (`KismetMathLibrary.DotProduct2D` (`KismetMathLibrary.Conv_VectorToVector2D` (`SceneComponent.GetForwardVector` (`self.CapsuleComponent`))) (`KismetMathLibrary.Conv_VectorToVector2D` KnockbackVector)) 0.0)
            (goto _label_4)))))))

(event `ResumePatrol`
  (`AITask_MoveTo.AIMoveTo` (`AIBlueprintHelperLibrary.GetAIController` self) (`SplineComponent.FindLocationClosestToWorldLocation` (`/Game/Characters/Enemies/Blueprints/BP_PatrolSpline.Spline` (`self.PatrolSpline`)) (`self.K2_GetActorLocation`) "World") null -1.0 "Default" "Default" true false
    (:`OnMoveFinished`
      (`self.StartPatrol`))))

(event `StartPatrol`
  (bind _spline (`/Game/Characters/Enemies/Blueprints/BP_PatrolSpline.Spline` (`self.PatrolSpline`)))
  (`KismetSystemLibrary.K2_ClearAndInvalidateTimerHandle` (`self.PatrolHandle`))
  (bind _returnvalue (`KismetSystemLibrary.K2_SetTimerDelegate` (delegate `Patrol`) 0.1 true true))
  (set `self.PatrolHandle` _returnvalue)
  (`AIController.MoveToLocation` (`AIBlueprintHelperLibrary.GetAIController` self) (`SplineComponent.GetLocationAtSplineInputKey` _spline (+ (`SplineComponent.FindInputKeyClosestToWorldLocation` _spline (`self.K2_GetActorLocation`)) 0.3) "World") -1.0 true true false true null true))

(event `Patrol`
  (bind _spline (`/Game/Characters/Enemies/Blueprints/BP_PatrolSpline.Spline` (`self.PatrolSpline`)))
  (bind _returnvalue (`AIController.MoveToLocation` (`AIBlueprintHelperLibrary.GetAIController` self) (`SplineComponent.GetLocationAtSplineInputKey` _spline (`SplineComponent.FindInputKeyClosestToWorldLocation` _spline (+ (`self.K2_GetActorLocation`) (* (`self.GetActorForwardVector`) 100.0))) "World") -1.0 true true false true null true))
  (switch `EPathFollowingRequestResult` _returnvalue
    (:`Failed`
      (`KismetSystemLibrary.PrintString` (`|GetEnumeratorNameAsString` _returnvalue)))))

(event `PrepareCharge`
  (`MovementComponent.StopMovementImmediately` (`self.CharacterMovement`))
  (`Controller.StopMovement` (`AIBlueprintHelperLibrary.GetAIController` self))
  (bind _returnvalue (`KismetSystemLibrary.K2_SetTimer` null "TrackPlayer" 0.033333 true true))
  (set `self.TrackingHandle` _returnvalue)
  (`KismetSystemLibrary.Delay` (`/Game/Characters/Enemies/PDA_ChargerEnemy.ChargeDuration` (`self.DataAsset`)))
  (`KismetSystemLibrary.K2_ClearAndInvalidateTimerHandle` (`self.TrackingHandle`))
  (`self.ChargeForward`))

(event `ChargeForward`
  (bind _returnvalue (`self.K2_GetActorLocation`))
  (bind _returnvalue_2 (+ _returnvalue (* (`self.GetActorForwardVector`) (`/Game/Characters/Enemies/PDA_ChargerEnemy.MaxDistance` (`self.DataAsset`)))))
  (bind (_outhit _returnvalue_3) (`KismetSystemLibrary.SphereTraceSingleForObjects` :`Start` _returnvalue :`End` _returnvalue_2 :`Radius` 20.0 :`ObjectTypes` (`|MakeArray` "ObjectTypeQuery17" "ObjectTypeQuery12" "ObjectTypeQuery1" :!type "EObjectTypeQuery Enum") :`DrawDebugType` "ForDuration"))
  (set `self.IsCharging` true)
  (if _returnvalue_3
    (set `self.TargetPoint` (`.Location` (`GameplayStatics.BreakHitResult` _outhit)))
    (else
      (set `self.TargetPoint` _returnvalue_2)))
  (bind _returnvalue_4 (`KismetSystemLibrary.K2_SetTimer` null "Charge" 0.033333 true true))
  (set `self.ChargeHandle` _returnvalue_4))

(event `HealthInterface.AddHealth`
  (params (Amount :type "Float (single-precision)"))
  (set `self.CurrentHealth` (`KismetMathLibrary.FClamp` (+ (`self.CurrentHealth`) Amount) 0.0 (`self.MaxHealth`))))

(event `HealthInterface.RemoveHealth`
  (params (Damage :type "Float (single-precision)") (EnemyRef :type "Actor Object Reference"))
  (bind _output_get (set `self.CurrentHealth` (`KismetMathLibrary.FClamp` (- (`self.CurrentHealth`) Damage) 0.0 (`self.MaxHealth`))))
  (if (<= _output_get 0.0)
    (`KismetSystemLibrary.DelayUntilNextTick`)
    (`self.K2_DestroyActor`)))

(fn `Charge`
  (`self.K2_SetActorLocation` (`KismetMathLibrary.VInterpTo_Constant` (`self.K2_GetActorLocation`) (`self.TargetPoint`) 0.033333 (`/Game/Characters/Enemies/PDA_ChargerEnemy.Speed` (`self.DataAsset`))) true)
  (if (< (`KismetMathLibrary.Vector_Distance` (`self.K2_GetActorLocation`) (`self.TargetPoint`)) (`/Game/Characters/Enemies/PDA_ChargerEnemy.StopMargin` (`self.DataAsset`)))
    (`self.InterruptCharge`)))

(fn `InterruptCharge`
  (`KismetSystemLibrary.K2_ClearAndInvalidateTimerHandle` (`self.ChargeHandle`))
  (set `self.IsCharging` false)
  (`self.Stun` (`/Game/Characters/Enemies/PDA_ChargerEnemy.AfterChargeWait` (`self.DataAsset`)) true))

(fn `ResetStun`
  (set `self.IsStunned` false)
  (`KismetSystemLibrary.K2_ClearAndInvalidateTimerHandle` (`self.StunHandle`))
  (bind _returnvalue (`KismetSystemLibrary.K2_SetTimer` null "TrackPlayer" 0.033333 true true))
  (set `self.TrackingHandle` _returnvalue)
  (`self.ResetCharge`))

(fn `TrackPlayer`
  (`self.K2_SetActorRotation` (`KismetMathLibrary.RInterpTo_Constant` (`self.K2_GetActorRotation`) (`KismetMathLibrary.FindLookAtRotation` (`self.K2_GetActorLocation`) (`self.K2_GetActorLocation` (`GameplayStatics.GetPlayerPawn` 0))) 0.033333 (`/Game/Characters/Enemies/PDA_ChargerEnemy.RotationRate` (`self.DataAsset`)))))

(fn `UserConstructionScript`)