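; Player vacuum weapon that sucks in BP_SuckableProp actors and fires them back out.
; VacuumTick line-traces props in a cone nearest first, pulling them by per-tag distance curves into a capped inventory, or onto a speed-changing handle if Heavy.
; BlowTick launches the held prop, or the newest stored one with a cooldown.
; Event dispatchers drive sound, VFX, shake and rumble, while a looping timer debug-draws the predicted shot path.
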(event `self.ReceiveBeginPlay`
  (`self.Init Feedback`))

(event `self.ReceiveTick`
  (params (DeltaSeconds :type "Float (single-precision)")))

(event `VacuumTick`
  (bind _cone_trigger_suck (`self.Cone Trigger Suck`))
  (bind _overlappingactors (`PrimitiveComponent.GetOverlappingActors` _cone_trigger_suck "/Game/BPs/VacuumProps/BP_SuckableProp.BP_SuckableProp_C"))
  (`|ExecutionSequence`
    (:`then_0`
      (`/Engine/EditorBlueprintResources/StandardMacros.IsValid` (`self.HeldActor`)
        (:`Is Not Valid`
          (`PrimitiveComponent.SetCollisionEnabled` _cone_trigger_suck "QueryOnly")
          (`|ExecutionSequence`
            (:`then_0`
              (bind _outarray (`StaticFunctions.OrderByDistance` (`GameplayStatics.GetPlayerCharacter` 0) _overlappingactors))
              (if (> (`KismetArrayLibrary.Array_Length` _overlappingactors) 0)
                (for _array_element _outarray
                  (set `self.IsVacuumingLarge` false)
                  (bind _asbp_suckable_prop (cast `/Game/BPs/VacuumProps/BP_SuckableProp` _array_element))
                  (bind _outhit (`KismetSystemLibrary.LineTraceSingleForObjects` (`SceneComponent.K2_GetComponentLocation` (`self.Muzzle`)) (`self.K2_GetActorLocation` _asbp_suckable_prop) (`|MakeArray` "ObjectTypeQuery1" "ObjectTypeQuery2" "ObjectTypeQuery3" "ObjectTypeQuery13" :!type "EObjectTypeQuery Enum") false (`|MakeArray` self (`GameplayStatics.GetPlayerPawn` 0) :!type "Actor Object Reference")))
                  (if (== (`.HitActor` (`GameplayStatics.BreakHitResult` _outhit)) _asbp_suckable_prop)
                    (if (not (`/Game/BPs/VacuumProps/BP_SuckableProp.DamageEnabled` _asbp_suckable_prop))
                      (bind _force (`self.GetForceValue` _asbp_suckable_prop))
                      (`self.Suck` _asbp_suckable_prop _force)
                      (if (< (`KismetMathLibrary.Vector_Distance` (`self.K2_GetActorLocation` _asbp_suckable_prop) (`SceneComponent.K2_GetComponentLocation` (`self.Muzzle`))) (`self.InventoryDistance`))
                        (if (`self.IsVacuumingLarge`)
                          (`self.SetHold` _asbp_suckable_prop)
                          (`|ExecutionSequence`
                            (:`then_0`
                              (set `self.IsVacuumingLarge` false)
                              (break))
                            (:`then_1`
                              (`self.On Prop Stucked` _asbp_suckable_prop)))
                          (else
                            (bind _full (`self.AddIntoInventory` _asbp_suckable_prop))
                            (`self.On Prop Sucked In` _asbp_suckable_prop _full)
                            (if _full
                              (bind _staticmesh (`/Game/BPs/VacuumProps/BP_SuckableProp.StaticMesh` _asbp_suckable_prop))
                              ; Temporary : Inventory full bounce
                              (`PrimitiveComponent.SetPhysicsLinearVelocity` _staticmesh (0.0 0.0 0.0) false "None")
                              (`PrimitiveComponent.AddImpulse` _staticmesh (+ (* (* (`KismetMathLibrary.Normal` (- (`self.K2_GetActorLocation` _asbp_suckable_prop) (`SceneComponent.K2_GetComponentLocation` (`self.Muzzle`)))) _force) 0.1) (0.0 0.0 200.0)) "None" true))))))))))
            (:`then_1`
              (for _array_element_2 (`PrimitiveComponent.GetOverlappingActors` (`self.Cone Trigger Suck`) null)
                (message `/Game/BPs/TestProps/BPI_VacuumReaction.ReactToVacuum` _array_element_2 (`KismetMathLibrary.Normal` (- (`self.K2_GetActorLocation`) (`self.K2_GetActorLocation` _array_element_2))))))))))
    (:`then_1`
      (`self.On Vacuum Tick`))))

(event `BlowTick`
  (bind _inventory (`self.Inventory`))
  (bind _returnvalue (`KismetArrayLibrary.Array_Length` _inventory))
  (`ActorComponent.Deactivate` (`self.NS_Vacuum_Spline`))
  (`/Engine/EditorBlueprintResources/StandardMacros.IsValid` (`self.HeldActor`)
    (:`Is Valid`
      (`self.ShootHeavy`))
    (:`Is Not Valid`
      (if (`self.CanShoot`)
        (if (> _returnvalue 0)
          (`self.Pre ShootLightMed` (`|GetArrayItem` _inventory (- _returnvalue 1)))
          (else
            ; Unlimited ammo
            (if (`self.DBG Unlimited Ammo`)
              (bind _returnvalue_2 (`|SpawnActorFromClass` "/Game/BPs/VacuumProps/BP_SuckableProp.BP_SuckableProp_C" (`KismetMathLibrary.MakeTransform` (0.0 0.0 0.0)) "Undefined" "MultiplyWithRoot" null null null))
              (`/Game/BPs/VacuumProps/BP_SuckableProp.Add to Inventory` _returnvalue_2 (0.0 0.0 0.0))
              (`self.Pre ShootLightMed` _returnvalue_2))))))))

(event `Pre ShootLightMed`
  (params (Prop :type "/Game/BPs/VacuumProps/BP_SuckableProp Object Reference"))
  (`|ExecutionSequence`
    (:`then_0`
      (`self.On Shoot` Prop))
    (:`then_1`
      (set `self.CanShoot` false)
      (`self.ShootLightMed` Prop)
      (`self.ResetCanShoot`))))

(event `Start Sucking`
  (`self.On Sucking State Change` true))

(event `Stop Sucking`
  (`|ExecutionSequence`
    (:`then_0`
      (bind _heldactor (`self.HeldActor`)
        (:`then`
          (`self.K2_DetachFromActor` _heldactor "KeepWorld" "KeepWorld" "KeepWorld")
          (bind _staticmesh (`/Game/BPs/VacuumProps/BP_SuckableProp.StaticMesh` _heldactor))
          (bind (_returnvalue_location _returnvalue_rotation) (`KismetMathLibrary.BreakTransform` (`SceneComponent.K2_GetComponentToWorld` _staticmesh)))
          (`SceneComponent.K2_SetWorldTransform` _staticmesh (`KismetMathLibrary.MakeTransform` _returnvalue_location _returnvalue_rotation) false false)
          (bind _staticmesh_2 (`/Game/BPs/VacuumProps/BP_SuckableProp.StaticMesh` _heldactor))
          (`PrimitiveComponent.SetSimulatePhysics` _staticmesh_2 true)
          (`PrimitiveComponent.SetCollisionEnabled` _staticmesh_2 "QueryAndPhysics")
          (set `self.HeldActor` null)
          (`/Game/Characters/Player/Blueprints/BP_Player.ResetSpeed` (cast `/Game/Characters/Player/Blueprints/BP_Player` (`GameplayStatics.GetPlayerCharacter` 0) :!pure true)))
        (:`else`)))
    (:`then_1`
      (`self.On Sucking State Change` false))))

(event `ResetCanShoot`
  (`/Engine/EditorBlueprintResources/StandardMacros.DoOnce` false :!label _label
    (:`Completed`
      (`KismetSystemLibrary.Delay` (`self.ShootDelay`))
      (set `self.CanShoot` true)
      (goto _label :!via `Reset`))))

(event `On Sucking State Change_Event` :!signature `self.On Sucking State Change`
  (params (State :type Boolean))
  (bind _ns_vacuum_spline (`self.NS_Vacuum_Spline`))
  (bind _ns_text_vrm (`self.NS_Text_VRM`))
  (if State
    ;[0 1 1] Start Sucking
    (`ActorComponent.Activate` _ns_vacuum_spline false)
    (`ActorComponent.Activate` _ns_text_vrm false)
    (bind _suckendsound (`self.SuckEndSound`)
      (:`then`
        (`AudioComponent.Stop` _suckendsound))
      (:`else`
        _))
    (bind _returnvalue (`GameplayStatics.SpawnSound2D` "/Game/_GameManager/Feedbacks/Sounds/Vacuum/A_Sucking_Start.A_Sucking_Start" 5.0 1.0 0.0 "/Game/_GameManager/Feedbacks/Sounds/SingleCancelPrevious_Vacuum_SC.SingleCancelPrevious_Vacuum_SC"))
    (set `self.SuckStartSound` _returnvalue)
    (`KismetSystemLibrary.Delay` (`self.VacuumStartToLoopDelay`))
    (set `self.CanPlayLoopSound` true)
    (else
      ;[0 1 1] Stop Sucking
      (`ActorComponent.Deactivate` _ns_vacuum_spline)
      (`ActorComponent.Deactivate` _ns_text_vrm)
      (bind _suckloopsound (`self.SuckLoopSound`)
        (:`then`
          (`AudioComponent.Stop` _suckloopsound)
          (bind _returnvalue_2 (`GameplayStatics.SpawnSound2D` "/Game/_GameManager/Feedbacks/Sounds/Vacuum/A_Sucking_End.A_Sucking_End" 5.0 1.0 0.0 null))
          (set `self.SuckEndSound` _returnvalue_2))
        (:`else`)))))

(event `Init Feedback`
  (`|ExecutionSequence`
    (:`then_0`
      (add `self.On Sucking State Change` (delegate `On Sucking State Change_Event`)))
    (:`then_1`
      (add `self.On Shoot` (delegate `On Shoot_Event`)))
    (:`then_2`
      (add `self.On Prop Sucked In` (delegate `On Prop Sucked In_Event`)))
    (:`then_3`
      (add `self.On Prop Stucked` (delegate `On Prop Stucked_Event`)))
    (:`then_4`
      (add `self.On Vacuum Tick` (delegate `On Vacuum Tick_Event`)))
    (:`then_5`
      (`KismetSystemLibrary.K2_SetTimer` null "PredictProjectilePath" 0.066667 true true))))

(event `On Shoot_Event` :!signature `self.On Shoot`
  (params (`Suckable Prop` :type "/Game/BPs/VacuumProps/BP_SuckableProp Object Reference"))
  (bind _returnvalue (`GameplayStatics.GetPlayerController` 0))
  (bind _ns_vacuum_burst (`self.NS_Vacuum_Burst`))
  (bind _ns_vacuum_burst_2 (`self.NS_Vacuum_Burst`))
  (`GameplayStatics.PlaySound2D` "/Game/_GameManager/Feedbacks/Sounds/Vacuum/A_Shoot.A_Shoot" 1.0 1.0 0.0 null null)
  (if (`self.ActorHasTag` `Suckable Prop` "Heavy")
    ;[0 1 1] Shoot FeedBacks (Heavy)
    (if (`/Game/_GameManager/GI_Systems.ControllerVibration?` (cast `/Game/_GameManager/GI_Systems` (`GameplayStatics.GetGameInstance`) :!pure true))
      (`PlayerController.K2_ClientPlayForceFeedback` (`GameplayStatics.GetPlayerController` 0) "/Game/_GameManager/Feedbacks/ForceFeedback/FFB_Vacuum_Suck_Light.FFB_Vacuum_Suck_Light" "None" false false false))
    (`ActorComponent.Activate` _ns_vacuum_burst false)
    (`KismetSystemLibrary.Delay` 0.2)
    (`ActorComponent.Deactivate` _ns_vacuum_burst)
    (else
      ;[0 1 1] Shoot Feedbacks (Light/Med)
      (`PlayerController.ClientStartCameraShake` :`self` _returnvalue :`Shake` "/Game/_GameManager/Feedbacks/CameraShake/BP_CameraShake_Suck.BP_CameraShake_Suck_C" :`Scale` 3.0)
      (if (`/Game/_GameManager/GI_Systems.ControllerVibration?` (cast `/Game/_GameManager/GI_Systems` (`GameplayStatics.GetGameInstance`) :!pure true))
        (`PlayerController.K2_ClientPlayForceFeedback` _returnvalue "/Game/_GameManager/Feedbacks/ForceFeedback/FFB_Vacuum_Suck_Light.FFB_Vacuum_Suck_Light" "None" false false false))
      (`SkeletalMeshComponent.PlayAnimation` (`self.SkeletalMesh`) "/Game/Characters/Player/Blueprints/Vacuum/Animation/AS_Vacuum_Blow_01.AS_Vacuum_Blow_01" false)
      (`ActorComponent.Activate` _ns_vacuum_burst_2 false)
      (`ActorComponent.Activate` (`self.NS_Text_POP`) false)
      (`KismetSystemLibrary.Delay` 0.2)
      (`ActorComponent.Deactivate` _ns_vacuum_burst_2)
      (`ActorComponent.Deactivate` (`self.NS_Text_POP`)))))

(event `On Prop Sucked In_Event` :!signature `self.On Prop Sucked In`
  (params (`Suckable Prop` :type "/Game/BPs/VacuumProps/BP_SuckableProp Object Reference") (`Inventory Is Full` :type Boolean))
  (if (not `Inventory Is Full`)
    (`SkeletalMeshComponent.PlayAnimation` (`self.SkeletalMesh`) "/Game/Characters/Player/Blueprints/Vacuum/Animation/AS_Vacuum_Suck_01.AS_Vacuum_Suck_01" false)))

(event `On Prop Stucked_Event` :!signature `self.On Prop Stucked`
  (params (`Suckable Prop` :type "/Game/BPs/VacuumProps/BP_SuckableProp Object Reference")))

(event `On Vacuum Tick_Event`
  (bind _returnvalue (`GameplayStatics.GetPlayerController` 0))
  ;[0 1 1] Suck Feedbacks loop
  (`PlayerController.ClientStartCameraShake` :`self` _returnvalue :`Shake` "/Game/_GameManager/Feedbacks/CameraShake/BP_CameraShake_Suck.BP_CameraShake_Suck_C")
  (if (`/Game/_GameManager/GI_Systems.ControllerVibration?` (cast `/Game/_GameManager/GI_Systems` (`GameplayStatics.GetGameInstance`) :!pure true))
    (`PlayerController.K2_ClientPlayForceFeedback` _returnvalue "/Game/_GameManager/Feedbacks/ForceFeedback/FFB_Vacuum_Suck_Light.FFB_Vacuum_Suck_Light" "None" false false false))
  (if (`self.CanPlayLoopSound`)
    (`self.SuckLoopSound`
      (:`then`)
      (:`else`
        (bind _returnvalue_2 (`GameplayStatics.SpawnSound2D` "/Game/_GameManager/Feedbacks/Sounds/Vacuum/A_Sucking_Loop.A_Sucking_Loop" 5.0 1.0 0.0 "/Game/_GameManager/Feedbacks/Sounds/SingleLoop_SC.SingleLoop_SC"))
        (`/Engine/EditorBlueprintResources/StandardMacros.IsValid` _returnvalue_2
          (:`Is Valid`
            (if (`AudioComponent.IsPlaying` _returnvalue_2)
              (set `self.SuckLoopSound` _returnvalue_2)
              (bind _suckstartsound (`self.SuckStartSound`)
                (:`then`
                  (`AudioComponent.Stop` _suckstartsound))
                (:`else`)))))))))

(fn `AddIntoInventory`
  (params (Prop :type "/Game/BPs/VacuumProps/BP_SuckableProp Object Reference"))
  (returns (Full :type Boolean))
  (bind _inventory (`self.Inventory`))
  (if (< (`KismetArrayLibrary.Array_Length` _inventory) (`self.InventoryMaxSize`))
    (`KismetArrayLibrary.Array_AddUnique` _inventory Prop)
    (set `self.LastPropMass` (`PrimitiveComponent.GetMass` (`/Game/BPs/VacuumProps/BP_SuckableProp.StaticMesh` Prop)))
    (`/Game/BPs/VacuumProps/BP_SuckableProp.Add to Inventory` Prop (`self.InventoryPosition`))
    (return false)
    (else
      (return true))))

(fn `Blow`)

(fn `GetForceValue`
  (params (Actor :type "Actor Object Reference"))
  (returns (Force :type "Float (double-precision)"))
  (return (`CurveFloat.GetFloatValue` (`BlueprintMapLibrary.Map_Find` (`self.ForceCurve`) (`|GetArrayItem` (`Actor.Tags` Actor))) (`KismetMathLibrary.Vector_Distance` (`self.K2_GetActorLocation` Actor) (`SceneComponent.K2_GetComponentLocation` (`self.Muzzle`))))))

(fn `PredictProjectilePath`
  (bind _inventory (`self.Inventory`))
  (if (`KismetArrayLibrary.Array_IsNotEmpty` _inventory)
    (`GameplayStatics.Blueprint_PredictProjectilePath_ByObjectType` (+ (`SceneComponent.K2_GetComponentLocation` (`self.Handle`)) (* (`SceneComponent.GetForwardVector` (`self.Arrow`)) 20.0)) (/ (* (`SceneComponent.GetForwardVector` (`self.Arrow`)) (select `bool` (`self.ActorHasTag` (`|GetArrayItem` _inventory (- (`KismetArrayLibrary.Array_Length` _inventory) 1)) "Light") :`false` (`self.BlowForceMedium`) :`true` (`self.BlowForceLight`))) (`self.LastPropMass`)) true 5.0 (`|MakeArray` "ObjectTypeQuery13" :!type "EObjectTypeQuery Enum") false (`|MakeArray` self (`GameplayStatics.GetPlayerPawn` 0) :!type "Actor Object Reference") "ForDuration" 0.066667 15.0 5.0)))

(fn `SetHold`
  (params (Prop :type "/Game/BPs/VacuumProps/BP_SuckableProp Object Reference"))
  (`PrimitiveComponent.SetSimulatePhysics` (`/Game/BPs/VacuumProps/BP_SuckableProp.StaticMesh` Prop) false)
  (`self.K2_AttachToComponent` Prop (`self.Handle`) "None" "SnapToTarget" "SnapToTarget" "SnapToTarget" false)
  (bind _output_get (set `self.HeldActor` Prop))
  (`PrimitiveComponent.SetCollisionEnabled` (`/Game/BPs/VacuumProps/BP_SuckableProp.StaticMesh` _output_get) "NoCollision")
  (`self.K2_SetActorRelativeTransform` _output_get (`KismetMathLibrary.MakeTransform` (`self.RelativeLocationHeld`) (`self.RelativeRotationHeld`)) false false)
  (`ActorComponent.Deactivate` (`self.NS_Vacuum_Spline`))
  (`/Game/Characters/Player/Blueprints/BP_Player.SetSpeedToHeld` (cast `/Game/Characters/Player/Blueprints/BP_Player` (`GameplayStatics.GetPlayerCharacter` 0) :!pure true)))

(fn `ShootHeavy`
  (bind _heldactor (`self.HeldActor`))
  (bind _heldactor_2 (`self.HeldActor`))
  (bind _staticmesh (`/Game/BPs/VacuumProps/BP_SuckableProp.StaticMesh` _heldactor_2))
  (bind _staticmesh_2 (`/Game/BPs/VacuumProps/BP_SuckableProp.StaticMesh` _heldactor_2))
  (bind (_returnvalue_location _returnvalue_rotation) (`KismetMathLibrary.BreakTransform` (`SceneComponent.K2_GetComponentToWorld` _staticmesh_2)))
  (`self.K2_DetachFromActor` _heldactor_2 "KeepWorld" "KeepWorld" "KeepWorld")
  (`SceneComponent.K2_SetWorldTransform` _staticmesh_2 (`KismetMathLibrary.MakeTransform` _returnvalue_location _returnvalue_rotation) false false)
  (`PrimitiveComponent.SetSimulatePhysics` _staticmesh true)
  (`PrimitiveComponent.SetCollisionEnabled` _staticmesh "QueryAndPhysics")
  (`/Game/BPs/VacuumProps/BP_SuckableProp.ActivateTrail` _heldactor)
  (`self.On Shoot` _heldactor)
  (`self.On Sucking State Change` false)
  (`/Game/BPs/VacuumProps/BP_SuckableProp.ResetHit` _heldactor)
  (`PrimitiveComponent.AddImpulse` (`/Game/BPs/VacuumProps/BP_SuckableProp.StaticMesh` _heldactor) (* (`SceneComponent.GetForwardVector` (`self.Arrow`)) (`self.BlowForceHeavy`)) "None" false)
  ;[1 0 0] Make this cleaner
  (bind _asbp_suckable_prop_aoe (cast `/Game/BPs/VacuumProps/BP_SuckableProp_AOE` (`self.HeldActor`))
    (:`then`
      (set `/Game/BPs/VacuumProps/BP_SuckableProp_AOE.IsActive` true _asbp_suckable_prop_aoe))
    (:`CastFailed`
      _))
  (set `self.HeldActor` null)
  (`self.ResetCanShoot`)
  (`/Game/Characters/Player/Blueprints/BP_Player.ResetSpeed` (cast `/Game/Characters/Player/Blueprints/BP_Player` (`GameplayStatics.GetPlayerCharacter` 0) :!pure true)))

(fn `ShootLightMed`
  (params (Prop :type "/Game/BPs/VacuumProps/BP_SuckableProp Object Reference"))
  (bind _staticmesh (`/Game/BPs/VacuumProps/BP_SuckableProp.StaticMesh` Prop))
  (bind _inventory (`self.Inventory`))
  (bind _returnvalue (`KismetArrayLibrary.Array_Length` _inventory))
  (bind _returnvalue_2 (`SceneComponent.GetForwardVector` (`self.Arrow`)))
  (`/Game/BPs/VacuumProps/BP_SuckableProp.Place to World` :`self` Prop :`Location` (+ (`SceneComponent.K2_GetComponentLocation` (`self.Handle`)) (* _returnvalue_2 20.0)))
  (`PrimitiveComponent.AddImpulse` _staticmesh (* _returnvalue_2 (select `bool` (`self.ActorHasTag` Prop "Light") :`false` (`self.BlowForceMedium`) :`true` (`self.BlowForceLight`))) "None" false)
  (`SceneComponent.K2_SetWorldRotation` _staticmesh (`KismetMathLibrary.RandomRotator` true) false false)
  (if (> _returnvalue 0)
    (`KismetArrayLibrary.Array_Remove` _inventory (- _returnvalue 1))))

(fn `Suck`
  (params (Actor :type "/Game/BPs/VacuumProps/BP_SuckableProp Object Reference") (Force :type "Float (double-precision)"))
  (`PrimitiveComponent.AddImpulse` (`/Game/BPs/VacuumProps/BP_SuckableProp.StaticMesh` Actor) (* (`KismetMathLibrary.Normal` (- (`SceneComponent.K2_GetComponentLocation` (`self.Muzzle`)) (`self.K2_GetActorLocation` Actor))) Force) "None" true)
  (if (`self.ActorHasTag` Actor "Heavy")
    (set `self.IsVacuumingLarge` true)))

(fn `UserConstructionScript`)