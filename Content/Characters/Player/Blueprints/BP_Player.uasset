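; First-person player character that dashes, kicks and carries a vacuum child actor, with health, post-hit immunity and death screen.
; DataAssetPlayer supplies tuning for movement, FOV, kick and vacuum inventory, including slower speeds for held objects.
; Kicks sphere-trace along pitch-clamped aim, message the hit actor and stretch a placeholder leg toward impact.
; Timelines and Tick drive PC_Systems screen-effect materials, while a looping timer emits pawn noise.
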(event Custom|AttacksCancel
  ;[0 0 0 0.4 75] Attack Systems
  ;;[0.15 0.15 0.15 0.5 50] Cancel attacks
  (Variables|Punch|Count|SetAttackType "NewEnumerator0")
  (Transformation|SetRelativeTransform (Variables|Default|GetKick_PlaceHolder) (Math|Transform|MakeTransform "0.000000,-40.000000,0.000000" "0.000000,-90.000000,0.000000" "1.000000,1.000000,1.000000") false false))

(event Custom|Hide%20Loading
  ;[0 0 0 0.4 75] BeginPlay
  ;;[0.15 0.15 0.15 0.5] Movement at the start & Loading Screen
  (Utilities|FlowControl|Delay 0.5))

(event Custom|SetSpeedToHeld
  (bind _charactermovement (Variables|Character|GetCharacterMovement))
  ;[0 0 0 0.4 75] Vacuum
  ;;[0.2262 0.9139 1 0.4 50] Change Speed when holding large obj
  (if (Actor|ActorHasTag (Variables|/Game/Characters/Player/Blueprints/BP_Vacuum.BP_Vacuum_C|GetHeldActor (.AsBP%20Vacuum (Utilities|Casting|CastToBP_Vacuum (Variables|/Script/Engine.ChildActorComponent|GetChildActor (Variables|Default|GetVacuum))))) "Medium")
    (Variables|/Script/Engine.CharacterMovementComponent|SetMaxWalkSpeed _charactermovement (Variables|/Game/_GameManager/Data_Assets/Data_3C/PDA_Player.PDA_Player_C|GetMediumObjectMoveSpeed (Variables|DataAsset|GetData_Asset_Player)))
    (else
      (Variables|/Script/Engine.CharacterMovementComponent|SetMaxWalkSpeed _charactermovement (Variables|/Game/_GameManager/Data_Assets/Data_3C/PDA_Player.PDA_Player_C|GetHeavyObjectMoveSpeed (Variables|DataAsset|GetData_Asset_Player))))))

(event Custom|ResetSpeed
  ;[0 0 0 0.4 75] Vacuum
  ;;[0.2262 0.9139 1 0.4 50] Change Speed when holding large obj
  (Variables|/Script/Engine.CharacterMovementComponent|SetMaxWalkSpeed (Variables|Character|GetCharacterMovement) (Variables|/Game/_GameManager/Data_Assets/Data_3C/PDA_Player.PDA_Player_C|GetMax_Walk_Speed (Variables|DataAsset|GetData_Asset_Player))))

(event Custom|Healing_Effect
  (bind _pc_systems (Variables|Refs|GetPC%20Systems))
  (bind _wbp_healing_effect (Variables|/Game/_GameManager/PC_Systems.PC_Systems_C|GetWBP%20Healing%20Effect _pc_systems))
  ;[0 0 0 0.4 75] Visual effect (VFX)
  ;;[0 1 0.1362 0.5 50] Heal Effect
  (bind _opacity_value (Timeline|Timeline_1 PlayFromStart)
    (:Update
      (Widget|SetRenderOpacity _wbp_healing_effect 1.0)
      (Rendering|Material|SetScalarParameterValue (Variables|/Game/UI/WBP_HealingEffect.WBP_HealingEffect_C|GetDynamicMat _wbp_healing_effect) "Anim" _opacity_value :!class /Script/Engine.MaterialInstanceDynamic))
    (:Finished
      (Widget|SetRenderOpacity _wbp_healing_effect 0.0))))

(event Custom|Kick
  (bind _returnvalue (Transformation|GetActorForwardVector))
  (bind _returnvalue_2 (Transformation|GetActorLocation))
  (bind _data_asset_player (Variables|DataAsset|GetData_Asset_Player))
  (bind _data_asset_player_2 (Variables|DataAsset|GetData_Asset_Player))
  (bind _data_asset_player_3 (Variables|DataAsset|GetData_Asset_Player))
  (bind _firstpersoncameracomponent (Variables|Default|GetFirstPersonCameraComponent))
  (bind _returnvalue_3 (Math|Vector|GetForwardVector _firstpersoncameracomponent))
  (bind _kick_force (Variables|/Game/_GameManager/Data_Assets/Data_3C/PDA_Player.PDA_Player_C|GetKick_Force _data_asset_player))
  (bind _kickcooldown (Variables|/Game/_GameManager/Data_Assets/Data_3C/PDA_Player.PDA_Player_C|GetKickCooldown _data_asset_player_2))
  (bind _returnvalue_4 (Math|Conversions|RotationFromXVector _returnvalue_3))
  (bind _returnvalue_5 (* _returnvalue (.x _kick_force)))
  ;[0 0 0 0.4 75] Kick
  ;;[0 1 0.3003 0.5 50] Kick
  (if (Variables|Default|GetCanKick)
    (Variables|Default|SetCanKick false)
    (Development|PrintString (Utilities|String|ToString(Float) _kickcooldown))
    (Utilities|Time|SetTimerbyEvent (delegate Custom|KickCooldownReset) _kickcooldown false true)
    (bind (_outhit _returnvalue_6) (Collision|SphereTraceForObjects _returnvalue_2 (+ _returnvalue_2 (* (Class|KismetMathLibrary|CreateVectorfromYawPitch (.yaw _returnvalue_4) (Math|Float|Clamp(Float) (.pitch _returnvalue_4) (Variables|/Game/_GameManager/Data_Assets/Data_3C/PDA_Player.PDA_Player_C|GetPitch%20Min _data_asset_player_3) (Variables|/Game/_GameManager/Data_Assets/Data_3C/PDA_Player.PDA_Player_C|GetPitch%20Max _data_asset_player_3)) 1.0) (Variables|/Game/_GameManager/Data_Assets/Data_3C/PDA_Player.PDA_Player_C|GetKick_Length (Variables|DataAsset|GetData_Asset_Player))) "") 2e+01 (Utilities|Array|MakeArray "ObjectTypeQuery3" "ObjectTypeQuery12" "ObjectTypeQuery14" "ObjectTypeQuery1" "ObjectTypeQuery2" "ObjectTypeQuery4" "ObjectTypeQuery19") false (Variables|Default|GetKickIgnoreList) "None"))
    (if _returnvalue_6
      (Development|PrintString (Utilities|GetDisplayName (.HitComponent (Collision|BreakHitResult _outhit))))
      (Class|KickedInterface|Kicked(Message) (.HitActor (Collision|BreakHitResult _outhit)) (Math|Vector|MakeVector (.x _returnvalue_5) (.y _returnvalue_5) (+ (.z _returnvalue_5) (Variables|/Game/_GameManager/Data_Assets/Data_3C/PDA_Player.PDA_Player_C|GetKick_Damage _data_asset_player))) (Transformation|GetActorLocation))
      (Class|HitInterface|GetHit(Message) (.HitActor (Collision|BreakHitResult _outhit)) (Variables|Default|Getdamage) 0.0 "0, 0, 0" 0.0 self)
      (CallFunction|KickFeedbackEvent (.ImpactPoint (Collision|BreakHitResult _outhit)) true)
      (else
        (CallFunction|KickFeedbackEvent (.TraceEnd (Collision|BreakHitResult _outhit)) false)))))

(event Custom|Hurt%20Effect
  (bind _pc_systems (Variables|Refs|GetPC%20Systems))
  (bind _wbp_hurt_screen_effect (Variables|/Game/_GameManager/PC_Systems.PC_Systems_C|GetWBP%20Hurt%20Screen%20Effect _pc_systems))
  ;[0 0 0 0.4 75] Visual effect (VFX)
  ;;[1 0 0 1 50] Hurt Effect
  (bind _opacity_value (Timeline|Timeline_0 PlayFromStart)
    (:Update
      (Widget|SetRenderOpacity _wbp_hurt_screen_effect 1.0)
      (Rendering|Material|SetScalarParameterValue (Variables|/Game/UI/WBP_HurtScreenEffect.WBP_HurtScreenEffect_C|GetDynamicMat _wbp_hurt_screen_effect) "Anim" _opacity_value :!class /Script/Engine.MaterialInstanceDynamic))
    (:Finished
      (Widget|SetRenderOpacity _wbp_hurt_screen_effect 0.0))))

(event Custom|Pre%20Attack%20Hit%20Notify
  (bind _capsulecomponent (Variables|Default|GetCapsuleComponent))
  (bind _returnvalue (Transformation|GetWorldLocation _capsulecomponent))
  ;[0 0 0 0.4 75] Attack Systems
  ;;[0 1 0 1 50] Pre Attack Hit Notify
  (bind _outhit (Collision|SphereTraceForObjects _returnvalue (+ _returnvalue (* (Math|Vector|GetForwardVector (Transformation|GetWorldRotation _capsulecomponent)) 6.5e+02)) 75.0 (Utilities|Array|MakeArray "ObjectTypeQuery3") false (Utilities|Array|MakeArray self) "ForDuration"))
  (bind _asbp_enemy (Utilities|Casting|CastToBP_Enemy (.HitActor (Collision|BreakHitResult _outhit))))
  (Default|PreAttackHit _asbp_enemy))

(event Custom|Start%20FOV
  ;[1 0.5179 0.9771 1 50] FOV Change For Dash
  (if (not (Variables|Dash|FOVEffect|GetHas%20Applied%20FOV))
    (Variables|Dash|FOVEffect|SetHas%20Applied%20FOV true)
    (Variables|Dash|FOVEffect|SetOld%20FOV (Variables|/Script/Engine.CameraComponent|GetFieldOfView (Variables|Default|GetFirstPersonCameraComponent)))
    (bind (_direction _fov_alpha) (Timeline|T_FOV Play)
      (:Update
        (Camera|SetFieldOfView (Variables|Default|GetFirstPersonCameraComponent) (Math|Float|Lerp (Variables|Dash|FOVEffect|GetOld%20FOV) (Variables|/Game/_GameManager/Data_Assets/Data_3C/PDA_Player.PDA_Player_C|GetDash_FOV (Variables|DataAsset|GetData_Asset_Player)) _fov_alpha)))
      (:Finished
        (if (Utilities|Enum|Equal(Enum) _direction "Backward")
          (Variables|Dash|FOVEffect|SetHas%20Applied%20FOV false))))))

(event Custom|StunState
  (bind _charactermovement (Variables|Character|GetCharacterMovement))
  (bind _pc_systems (Variables|Refs|GetPC%20Systems))
  (bind _stunwidget (Variables|/Game/_GameManager/PC_Systems.PC_Systems_C|GetStunWidget _pc_systems))
  ;[0 0 0 0.4 75] Visual effect (VFX)
  ;;[0.6667 0.6667 0.6667 0.5 50] Stun State & Effect
  (Variables|Default|SetbCanDash false)
  (Components|Movement|StopMovementImmediately _charactermovement)
  (Variables|/Script/Engine.CharacterMovementComponent|SetMaxWalkSpeed _charactermovement 0.0)
  (bind _opacity_value (Timeline|StunState_TL PlayFromStart)
    (:Update
      (Widget|SetRenderOpacity _stunwidget 1.0)
      (Rendering|Material|SetScalarParameterValue (Variables|/Game/UI/WBP_Stun.WBP_Stun_C|GetDynamicMat _stunwidget) "Anim" _opacity_value :!class /Script/Engine.MaterialInstanceDynamic))
    (:Finished
      (Variables|/Script/Engine.CharacterMovementComponent|SetMaxWalkSpeed (Variables|Character|GetCharacterMovement) (Variables|/Game/_GameManager/Data_Assets/Data_3C/PDA_Player.PDA_Player_C|GetMax_Walk_Speed (Variables|DataAsset|GetData_Asset_Player)))
      (Widget|SetRenderOpacity _stunwidget 0.0)
      (Variables|Default|SetbCanDash true))))

(event Custom|Dead
  (bind _returnvalue (Game|GetPlayerController 0))
  (bind _returnvalue_2 (Game|GetGameInstance))
  (bind _capsulecomponent (Variables|Default|GetCapsuleComponent))
  (bind _aspc_systems (Utilities|Casting|CastToPC_Systems _returnvalue))
  (bind _asgi_systems (Utilities|Casting|CastToGI_Systems _returnvalue_2))
  (bind _wbp_death_screen (Variables|/Game/_GameManager/PC_Systems.PC_Systems_C|GetWBP%20Death%20Screen _aspc_systems))
  ;[0 0 0 0.4 75] HP Systems
  ;;[1 0 0 1 50] Death
  (Collision|SetCollisionResponsetoChannel _capsulecomponent "ECC_GameTraceChannel14" "ECR_Ignore")
  (Collision|SetCollisionResponsetoChannel _capsulecomponent "ECC_GameTraceChannel13" "ECR_Ignore")
  (Collision|SetCollisionResponsetoChannel _capsulecomponent "ECC_GameTraceChannel4" "ECR_Ignore")
  (Pawn|Components|CharacterMovement|SetMovementMode (Variables|Character|GetCharacterMovement) "MOVE_None" 0)
  (Widget|SetVisibility _wbp_death_screen "Visible")
  (Input|SetInputModeUIOnly (Game|GetPlayerController 0) (Variables|/Game/UI/WBP_DeathScreen.WBP_DeathScreen_C|GetRetryLevelButton _wbp_death_screen) "DoNotLock" false)
  (bind _newtrack_0 (Timeline|Opacity_TL PlayFromStart)
    (:Update
      (Variables|/Script/UMG.Widget|SetRenderOpacity _wbp_death_screen _newtrack_0))
    (:Finished
      (Default|PauseTimer _asgi_systems)
      (Variables|/Game/_GameManager/GI_Systems.GI_Systems_C|SetElapsedTime _asgi_systems 0.0))))

(event Custom|Stop%20FOV
  ;[1 0.5179 0.9771 1 50] FOV Change For Dash
  (if (Variables|Dash|FOVEffect|GetHas%20Applied%20FOV)
    (bind (_direction _fov_alpha) (Timeline|T_FOV Reverse)
      (:Update
        (Camera|SetFieldOfView (Variables|Default|GetFirstPersonCameraComponent) (Math|Float|Lerp (Variables|Dash|FOVEffect|GetOld%20FOV) (Variables|/Game/_GameManager/Data_Assets/Data_3C/PDA_Player.PDA_Player_C|GetDash_FOV (Variables|DataAsset|GetData_Asset_Player)) _fov_alpha)))
      (:Finished
        (if (Utilities|Enum|Equal(Enum) _direction "Backward")
          (Variables|Dash|FOVEffect|SetHas%20Applied%20FOV false))))))

(event Custom|KickCooldownReset
  (Variables|Default|SetCanKick true))

(event Input|EnhancedActionEvents|EnhancedInputActionIA_Dash
  (params (ActionValue :type Boolean) (ElapsedSeconds :type Float%20%28double-precision%29) (TriggeredSeconds :type Float%20%28double-precision%29) (InputAction :type Input%20Action%20Object%20Reference :default "/Game/_GameManager/Inputs/Actions/IA_Dash.IA_Dash"))
  (bind _returnvalue (Class|Pawn|GetLastMovementInputVector))
  (bind _charactermovement (Variables|Character|GetCharacterMovement))
  (bind _data_asset_player (Variables|DataAsset|GetData_Asset_Player))
  (bind _charactermovement_2 (Variables|Character|GetCharacterMovement))
  (bind _dash_distance (Variables|/Game/_GameManager/Data_Assets/Data_3C/PDA_Player.PDA_Player_C|GetDash_Distance _data_asset_player))
  (bind _returnvalue_2 (* _dash_distance 1e+01))
  ;[0 0 0 0.5 75] Dash
  ;;[0.5873 1 0.002117 1 50] Dash
  (if (Variables|Default|GetbCanDash)
    (CallFunction|AttacksCancel)
    ;;[0 0 1 0.5 30] Debug
    (Variables|Dash|SetDashStartLocation (Transformation|GetWorldLocation (Variables|Default|GetCapsuleComponent)))
    (Variables|Dash|SetDashStartFrame (Utilities|GetFrameCount))
    (Variables|Default|SetbCanDash false)
    (Variables|Default|SetisDashing true)
    (Variables|Dash|SetOld%20Velocity (Variables|/Script/Engine.MovementComponent|GetVelocity _charactermovement))
    (Variables|Dash|SetOld%20Ground%20Friction (Variables|/Script/Engine.CharacterMovementComponent|GetGroundFriction _charactermovement))
    (Variables|/Script/Engine.CharacterMovementComponent|SetGroundFriction _charactermovement 0.0)
    (if (Math|Vector|VectorIsNearlyZero _returnvalue)
      (Variables|/Script/Engine.MovementComponent|SetVelocity _charactermovement (* (* (Transformation|GetActorForwardVector) -1.0) _returnvalue_2))
      (else
        (Variables|/Script/Engine.MovementComponent|SetVelocity _charactermovement (* (Math|Vector|Normalize _returnvalue) _returnvalue_2))))
    (CallFunction|StartFOV)
    (Utilities|FlowControl|Delay (Variables|/Game/_GameManager/Data_Assets/Data_3C/PDA_Player.PDA_Player_C|GetDash_Duration (Variables|DataAsset|GetData_Asset_Player)))
    (CallFunction|StopFOV)
    (Variables|Default|SetisDashing false)
    (Variables|/Script/Engine.CharacterMovementComponent|SetGroundFriction _charactermovement_2 (Variables|Dash|GetOld%20Ground%20Friction))
    (Variables|/Script/Engine.MovementComponent|SetVelocity _charactermovement_2 (Variables|Dash|GetOld%20Velocity))
    ;[0 0 1 0.5 30] Debug
    (Development|PrintText (Utilities|Text|FormatText "Dash distance : {dis} meters; duration : {tim} frames" (/ (Math|Vector|Distance(Vector) (Transformation|GetWorldLocation (Variables|Default|GetCapsuleComponent)) (Variables|Dash|GetDashStartLocation)) 1e+02) (- (Utilities|GetFrameCount) (Variables|Dash|GetDashStartFrame))) true true "(R=0.000000,G=0.660000,B=1.000000,A=1.000000)" 5.0)
    (Utilities|FlowControl|Delay (Variables|/Game/_GameManager/Data_Assets/Data_3C/PDA_Player.PDA_Player_C|GetDash_Cooldown (Variables|DataAsset|GetData_Asset_Player)))
    (Variables|Default|SetbCanDash true)))

(event EventAddHealth
  (params (Amount :type Float%20%28single-precision%29))
  ;[0 0 0 0.4 75] HP Systems
  ;;[0 0.15 0.03145 0.5 50] Health Systems
  (Variables|Default|SetCurrentHealth (Math|Float|Clamp(Float) (+ (Variables|Default|GetCurrentHealth) Amount) 0.0 (Variables|Default|GetMaxHealth)))
  (CallFunction|HealingEffect))

(event EventBeginPlay
  (bind _kickignorelist (Variables|Default|GetKickIgnoreList))
  ;[0 0 0 0.4 75] BeginPlay
  (Utilities|FlowControl|Sequence
    (:then_0
      (DataAsset|SetDataAsset)
      (CallFunction|InitFeedback)
      (|CallParentFunction))
    (:then_1
      (bind _aspc_systems (Utilities|Casting|CastToPC_Systems (Pawn|GetController))
        (:then
          (Variables|Refs|SetPC%20Systems _aspc_systems))
        (:CastFailed
          (Development|PrintString "Player: PC System fail" true true "(R=1.000000,G=0.000000,B=0.000000,A=1.000000)" 1e+01))))
    (:then_2
      (Camera|SetFieldOfView (Variables|Default|GetFirstPersonCameraComponent) (Variables|/Game/_GameManager/Data_Assets/Data_3C/PDA_Player.PDA_Player_C|GetCurrent_FOV (Variables|DataAsset|GetData_Asset_Player)))
      (Utilities|FlowControl|DelayUntilNextTick)
      (Transformation|SetWorldLocation (Variables|/Game/Characters/Player/Blueprints/BP_Vacuum.BP_Vacuum_C|GetMuzzle (.AsBP%20Vacuum (Utilities|Casting|CastToBP_Vacuum (Variables|/Script/Engine.ChildActorComponent|GetChildActor (Variables|Default|GetVacuum))))) (Transformation|GetWorldLocation (Variables|Default|GetPlayerMuzzleTransform)) false false)
      (Utilities|Array|Add _kickignorelist self)
      (Utilities|Array|Add _kickignorelist (Variables|/Script/Engine.ChildActorComponent|GetChildActor (Variables|Default|GetVacuum)))
      (Utilities|Time|SetTimerbyFunctionName 0 "MakeNoiseCall" 0.1 true))
    (:then_3
      ;;[0.15 0.15 0.15 0.5] Movement at the start & Loading Screen
      (if (Variables|Default|GetWaitForLoad)
        (Pawn|Components|CharacterMovement|DisableMovement (Variables|Character|GetCharacterMovement))
        (Utilities|FlowControl|Delay (+ (Variables|Default|GetLoading_Duration) 0.25)))
      (Widget|SetVisibility (Variables|/Game/_GameManager/PC_Systems.PC_Systems_C|GetWBp%20Loading%20Screen (.AsPC%20Systems (Utilities|Casting|CastToPC_Systems (Pawn|GetController)))) "Hidden")
      (Variables|/Script/Engine.CharacterMovementComponent|SetDefaultLandMovementMode (Variables|Character|GetCharacterMovement) "MOVE_Walking")
      (bind _returnvalue (Game|GetCurrentLevelName true))
      (if (Utilities|Enum|Equal(Enum) _returnvalue "L_Persistent")
        (bind _outactors (Actor|GetAllActorsOfClass "/Script/Engine.PlayerStart"))
        (bind _array_element (Utilities|Array|ForEachLoopwithBreak _outactors :!label _label)
          (:LoopBody
            (if (not (Actor|ActorHasTag _array_element "START_PERSISTENT"))
              (Transformation|SetActorTransform (Transformation|GetActorTransform _array_element) false true)
              (goto _label Break))))))
    (:then_4
      (bind _asgi_systems (Utilities|Casting|CastToGI_Systems (Game|GetGameInstance))
        (:then
          (Variables|Default|SetGame%20Instance _asgi_systems))
        (:CastFailed
          (Development|PrintString "Player: GI System fail" true true "(R=1.000000,G=0.000000,B=0.000000,A=1.000000)" 1e+01))))
    (:then_5
      (Utilities|FlowControl|Delay 5.0)
      (bind _outactors_2 (Actor|GetAllActorsOfClass "/Game/BPs/Arena/BP_Arena.BP_Arena_C"))
      (Utilities|Array|AppendArray (Variables|Default|GetKickIgnoreList) _outactors_2)
      (bind _outactors_3 (Actor|GetAllActorsOfClass "/Game/BPs/Bp_Pressure_Plate.Bp_Pressure_Plate_C"))
      (Utilities|Array|AppendArray (Variables|Default|GetKickIgnoreList) _outactors_3))))

(event EventMapSettingsDataBlueprint
  ;[0 0 0 0.3 75] Player Data To Settings
  (Variables|/Game/_GameManager/Data_Assets/Data_3C/PDA_Player.PDA_Player_C|SetCamera_Horizontal_Speed (Variables|/Game/_GameManager/PC_Systems.PC_Systems_C|GetData_Asset_Player (Variables|Refs|GetPC%20Systems)) (Class|SettingsSave|GetHorizontalSensitivity (Variables|Default|GetSettingsSave)))
  (Variables|/Game/_GameManager/Data_Assets/Data_3C/PDA_Player.PDA_Player_C|SetCamera_Vertical_Speed (Variables|/Game/_GameManager/PC_Systems.PC_Systems_C|GetData_Asset_Player (Variables|Refs|GetPC%20Systems)) (Class|SettingsSave|GetVerticalSensitivity (Variables|Default|GetSettingsSave))))

(event EventRemoveHealth
  (params (Damage :type Float%20%28single-precision%29) (EnemyRef :type Actor%20Object%20Reference))
  ;[0 0 0 0.4 75] HP Systems
  ;;[0 0.15 0.03145 0.5 50] Health Systems
  (if (not (Variables|Default|GetInvicible))
    (bind _output_get (Variables|Default|SetCurrentHealth (Math|Float|Clamp(Float) (- (Variables|Default|GetCurrentHealth) Damage) 0.0 (Variables|Default|GetMaxHealth))))
    (CallFunction|HurtEffect)
    (if (<= _output_get 0.0)
      (CallFunction|Dead)
      (else
        (bind _foundwidgets (Widget|GetAllWidgetsOfClass "/Game/UI/Menus/InGameMenu/WBP_InGameMenu.WBP_InGameMenu_C" true))
        (Default|OnHit (Utilities|Array|Get(acopy) _foundwidgets) EnemyRef)))))

(event EventTick
  (params (DeltaSeconds :type Float%20%28single-precision%29))
  ;[0 0 0 0.4 75] Event Tick
  (Utilities|FlowControl|Sequence
    (:then_0
      (CallFunction|DamageEffect))))

(event EventGetHit
  (params (Damage :type Float%20%28single-precision%29) (HitStunDuration :type Float%20%28single-precision%29) (KnockbackVector :type Vector :default "0, 0, 0") (InvincibilityTime :type Float%20%28single-precision%29) (SourceActor :type Actor%20Object%20Reference))
  ;[0 0 0 0.4 75] HP Systems
  ;;[1 0.2455 0.000893 0.5 50] GetHit
  (if (not (Variables|Default|GetPostHit%20Immune))
    (Utilities|FlowControl|Sequence
      (:then_0
        (Class|HealthInterface|RemoveHealth Damage SourceActor)
        (Variables|Default|SetPostHit%20Immune true)
        (bind _returnvalue (Utilities|Time|SetTimerbyFunctionName 0 "InvinsibilityReset" (Math|Float|Max(Float) InvincibilityTime 0.01) false true))
        (Variables|Default|SetInvinsibilityTimer _returnvalue))
      (:then_1
        (CallFunction|GettingHitFBEvent)))))

(event Input|KeyboardEvents|DebugKeyO
  (params (Key :type Key%20Structure :default "None") (ActionValue :type Input%20Action%20Value%20Structure))
  ;[0 0 0 0.4 75] Debug Key
  (:Released
    (Class|FTJScoringSystemScore|IncreasewithText (Subsystems|GetBPScoringSystemScore) 10 0 (Utilities|Text|FormatText "Score test"))))

(event Input|KeyboardEvents|DebugKeyAdd
  (params (Key :type Key%20Structure :default "None") (ActionValue :type Input%20Action%20Value%20Structure))
  ;[0 0 0 0.4 75] Debug Key
  (:Pressed
    (Class|HealthInterface|AddHealth 1e+01)))

(event Input|KeyboardEvents|DebugKeySubtract
  (params (Key :type Key%20Structure :default "None") (ActionValue :type Input%20Action%20Value%20Structure))
  ;[0 0 0 0.4 75] Debug Key
  (:Pressed
    (Class|HealthInterface|RemoveHealth 1e+01)))

(event Custom|Init%20Feedback
  (Utilities|FlowControl|Sequence
    (:then_0
      ;[0 0 0 0.4 75] Getting Hit
      (EventDispatchers|BindEventtoGettingHitFB (delegate Custom|Getting_Hit_FB_Event)))
    (:then_1
      ;[0 0 0 0.4 75] Kick Feedback
      (EventDispatchers|BindEventtoKickFeedback (delegate Custom|Kick_Feedback_Event)))))

(event Custom|Getting_Hit_FB_Event
  (bind _returnvalue (Game|GetPlayerController 0))
  ;[0 0 0 0.4 75] Getting Hit
  ;;[0 1 1] FB - Vibration & Camera Shake
  (if (Variables|/Game/_GameManager/GI_Systems.GI_Systems_C|GetControllerVibration? (Variables|Default|GetGame%20Instance))
    (Game|Feedback|ClientStartCameraShake _returnvalue "/Game/VFX/Blueprint/BP_FX_CameraShake_Impact_Strong.BP_FX_CameraShake_Impact_Strong_C" 1.0 "CameraLocal" "0, 0, 0")
    (Game|Feedback|PlayDynamicForceFeedback _returnvalue 1.0 0.2 true true true true)))

(event Custom|Kick_Feedback_Event
  (params (HitLocation :type Vector) (Hit_Something :type Boolean))
  (bind _returnvalue (Game|GetPlayerController 0))
  (bind _kick_placeholder (Variables|Default|GetKick_PlaceHolder))
  (bind _relativescale3d (Variables|/Script/Engine.SceneComponent|GetRelativeScale3D _kick_placeholder))
  ;[0 0 0 0.4 75] Kick Feedback
  ;;[0.005858 1 1 0.5] FB - SFX Kick
  (Audio|PlaySound2D (Variables|Feedback|GetSound_When_Kick) 0.5 1.0 0.0 0 0 false)
  (Rendering|SetVisibility (Variables|Default|GetKick_PlaceHolder) true false)
  (if (Variables|/Game/_GameManager/GI_Systems.GI_Systems_C|GetControllerVibration? (Variables|Default|GetGame%20Instance))
    ;;[0.005858 1 1 0.5] FB - Camera Shake & Vibration
    (Game|Feedback|ClientPlayForceFeedback _returnvalue "/Game/_GameManager/Feedbacks/ForceFeedback/FFB_Kick.FFB_Kick" "None" false false false))
  (Game|Feedback|ClientStartCameraShake _returnvalue "/Game/_GameManager/Feedbacks/CameraShake/BP_CameraShake_Kick.BP_CameraShake_Kick_C" 1.0 "World" "0, 0, 0")
  (Transformation|SetRelativeLocation (Variables|Default|GetKickLocation) (- HitLocation (Transformation|GetActorLocation)) false false)
  (Components|Timeline|SetPlayRate (Variables|Default|GetT_Kick1) (/ 1.0 (Variables|Kick|GetKickAnimDuration)))
  (Utilities|FlowControl|DelayUntilNextTick)
  (bind (_direction _kick_length_transition _kick_rotate_transition) (Timeline|T_Kick1 PlayFromStart)
    (:Update
      (Transformation|SetRelativeScale3D (Variables|Default|GetKick_PlaceHolder) (Math|Vector|MakeVector (.x _relativescale3d) (.y _relativescale3d) (Math|Float|Lerp 1.0 (/ (Math|Vector|Distance(Vector) (Transformation|GetWorldLocation (Variables|Default|GetKickLocation)) (Transformation|GetActorLocation)) 95.0) _kick_length_transition)))
      (bind _result (Math|Float|NegateFloat (Math|Float|Lerp 0.0 (+ (Math|Float|Clamp(Float) (.pitch (Transformation|GetWorldRotation (Variables|Default|GetFirstPersonCameraComponent))) -8e+01 1e+01) 9e+01) _kick_rotate_transition))
        (:%20%20
          (Transformation|SetRelativeRotation (Variables|Default|GetKick_PlaceHolder) (Math|Rotator|MakeRotator _result (Variables|Default|GetKickFootAngle) -9e+01) false false)
          (if Hit_Something
            (Utilities|FlowControl|DoOnce false :!label _label
              (:Completed
                ;;[0.005858 1 1 0.5] FB - VFX Kick Hit
                (bind _returnvalue_2 (Niagara|SpawnSystematLocation "/Game/VFX/Niagara/Kick/NS_Kick_Normal.NS_Kick_Normal" HitLocation))
                (if (Variables|/Game/_GameManager/GI_Systems.GI_Systems_C|GetControllerVibration? (Variables|Default|GetGame%20Instance))
                  (Game|Feedback|PlayDynamicForceFeedback (Game|GetPlayerController 0) 0.2 0.2 true true true true))
                (Utilities|FlowControl|Delay 0.4)
                (Components|DestroyComponent _returnvalue_2)
                (goto _label Reset)))))))
    (:Finished
      (Rendering|SetVisibility (Variables|Default|GetKick_PlaceHolder) false false))))

(fn ConstructionScript)

(fn SetSpeed/Accel/RotaRate
  (params (Max%20Walk%20Speed :type Float%20%28double-precision%29) (Max%20Acceleration :type Float%20%28double-precision%29) (Rotation%20Rate :type Rotator))
  (bind _charactermovement (Variables|Character|GetCharacterMovement))
  (Variables|/Script/Engine.CharacterMovementComponent|SetMaxWalkSpeed _charactermovement Max%20Walk%20Speed)
  (Variables|/Script/Engine.CharacterMovementComponent|SetMaxAcceleration _charactermovement Max%20Acceleration)
  (Variables|/Script/Engine.CharacterMovementComponent|SetRotationRate _charactermovement Rotation%20Rate))

(fn SetDataAsset
  (Utilities|FlowControl|Sequence
    (:then_0
      (Variables|/Script/Engine.CharacterMovementComponent|SetMaxWalkSpeed (Variables|Character|GetCharacterMovement) (Variables|/Game/_GameManager/Data_Assets/Data_3C/PDA_Player.PDA_Player_C|GetMax_Walk_Speed (Variables|DataAsset|GetData_Asset_Player))))
    (:then_2
      (bind _asbp_vacuum (Utilities|Casting|CastToBP_Vacuum (Variables|/Script/Engine.ChildActorComponent|GetChildActor (Variables|Default|GetVacuum)))
        (:then
          (Variables|/Game/Characters/Player/Blueprints/BP_Vacuum.BP_Vacuum_C|SetInventoryMaxSize _asbp_vacuum (Variables|/Game/_GameManager/Data_Assets/Data_3C/PDA_Player.PDA_Player_C|GetInventoryMaxSize (Variables|DataAsset|GetData_Asset_Player))))
        (:CastFailed
          (Development|PrintString "Player::SetDataAsset Failed to Cast BP_Vacuum" true true "(R=1.000000,G=0.000000,B=0.000000,A=1.000000)" 3e+01))))))

(fn DamageEffect
  (bind _currenthealth (Variables|Default|GetCurrentHealth))
  (bind _pc_systems (Variables|Refs|GetPC%20Systems))
  (bind _pc_systems_2 (Variables|Refs|GetPC%20Systems))
  (bind _pc_systems_3 (Variables|Refs|GetPC%20Systems))
  (bind _pc_systems_4 (Variables|Refs|GetPC%20Systems))
  (bind _wbp_damage_effect (Variables|/Game/_GameManager/PC_Systems.PC_Systems_C|GetWBP%20Damage%20Effect _pc_systems))
  (bind _wbp_damage_effect_2 (Variables|/Game/_GameManager/PC_Systems.PC_Systems_C|GetWBP%20Damage%20Effect _pc_systems_2))
  (bind _wbp_damage_effect_3 (Variables|/Game/_GameManager/PC_Systems.PC_Systems_C|GetWBP%20Damage%20Effect _pc_systems_3))
  (bind _wbp_damage_effect_4 (Variables|/Game/_GameManager/PC_Systems.PC_Systems_C|GetWBP%20Damage%20Effect _pc_systems_4))
  (bind _dynamicmat (Variables|/Game/UI/WBP_DamagePurcentEffect.WBP_DamagePurcentEffect_C|GetDynamicMat _wbp_damage_effect))
  (bind _dynamicmat_2 (Variables|/Game/UI/WBP_DamagePurcentEffect.WBP_DamagePurcentEffect_C|GetDynamicMat _wbp_damage_effect_2))
  (bind _dynamicmat_3 (Variables|/Game/UI/WBP_DamagePurcentEffect.WBP_DamagePurcentEffect_C|GetDynamicMat _wbp_damage_effect_3))
  (bind _dynamicmat_4 (Variables|/Game/UI/WBP_DamagePurcentEffect.WBP_DamagePurcentEffect_C|GetDynamicMat _wbp_damage_effect_4))
  (if (> _currenthealth 1e+01)
    (if (> _currenthealth 3e+01)
      (if (> _currenthealth 5e+01)
        (Rendering|Material|SetScalarParameterValue _dynamicmat "Anim" 0.0 :!class /Script/Engine.MaterialInstanceDynamic)
        (Rendering|Material|SetScalarParameterValue _dynamicmat "HeartBeat_Speed" 0.0 :!class /Script/Engine.MaterialInstanceDynamic)
        (else
          (Rendering|Material|SetScalarParameterValue _dynamicmat_2 "Anim" 1.0 :!class /Script/Engine.MaterialInstanceDynamic)
          (Rendering|Material|SetScalarParameterValue _dynamicmat_2 "CurveOffset" 0.0 :!class /Script/Engine.MaterialInstanceDynamic)
          (Rendering|Material|SetScalarParameterValue _dynamicmat_2 "Transition" 1.2 :!class /Script/Engine.MaterialInstanceDynamic)
          (Rendering|Material|SetScalarParameterValue _dynamicmat_2 "HeartBeat_Speed" 0.0 :!class /Script/Engine.MaterialInstanceDynamic)))
      (else
        (Rendering|Material|SetScalarParameterValue _dynamicmat_3 "Anim" 1.0 :!class /Script/Engine.MaterialInstanceDynamic)
        (Rendering|Material|SetScalarParameterValue _dynamicmat_3 "Transition" 0.5 :!class /Script/Engine.MaterialInstanceDynamic)
        (Rendering|Material|SetScalarParameterValue _dynamicmat_3 "HeartBeat_Speed" 0.0 :!class /Script/Engine.MaterialInstanceDynamic)))
    (else
      (Rendering|Material|SetScalarParameterValue _dynamicmat_4 "Anim" 1.0 :!class /Script/Engine.MaterialInstanceDynamic)
      (Rendering|Material|SetScalarParameterValue _dynamicmat_4 "CurveOffset" 1e+01 :!class /Script/Engine.MaterialInstanceDynamic)
      (Rendering|Material|SetScalarParameterValue _dynamicmat_4 "Transition" 0.0 :!class /Script/Engine.MaterialInstanceDynamic)
      (Rendering|Material|SetScalarParameterValue _dynamicmat_4 "HeartBeat_Speed" 1.25 :!class /Script/Engine.MaterialInstanceDynamic))))

(fn InvinsibilityReset
  (Variables|Default|SetPostHit%20Immune false)
  (Utilities|Time|ClearandInvalidateTimerbyHandle (Variables|Default|GetInvinsibilityTimer)))

(fn MakeNoiseCall
  (Class|PawnNoiseEmitterComponent|MakeNoise (Variables|Default|GetPawnNoiseEmitter) self 1.0 (Transformation|GetActorLocation)))