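; Base progress Blueprint that routes dialogue and end-screen requests to the UI widgets held by the given player controller.
; Dialogue looks up a row in DT_Dialogues and shows it in either the in-game or cinematic dialogue widget, depending on a flag.
; EndText collapses the cinematic box, and ForceEnd shows the end screen.
; Initialization starts a looping one-second timer on Update, which is currently empty.
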(event `self.InitializeBlueprint`
  (`parent.InitializeBlueprint`)
  (`KismetSystemLibrary.K2_SetTimer` null "Update" 1.0 true true))

(event `self.DeinitializeBlueprint`
  (`parent.DeinitializeBlueprint`))

(event `Dialogue`
  (params (PlayerController :type "/Game/_GameManager/PC_Systems Object Reference") (RowName :type Name) (`In Game Dialogue` :type Boolean))
  (if `In Game Dialogue`
    (bind _returnvalue (`|GetDataTableRow` "/Game/_GameManager/Data_Assets/Dialogues/DT_Dialogues.DT_Dialogues" RowName)
      (:`then`
        (`/Game/UI/Menus/InGameMenu/WBP_Dialogue_In_Game.DisplayDialogue` (`/Game/_GameManager/PC_Systems.WBP Dialogue in Game` PlayerController) _returnvalue)))
    (else
      (bind _returnvalue_2 (`|GetDataTableRow` "/Game/_GameManager/Data_Assets/Dialogues/DT_Dialogues.DT_Dialogues" RowName)
        (:`then`
          (`/Game/UI/Menus/InGameMenu/WBP_Dialogue_Cinematic.DisplayDialogue` (`/Game/_GameManager/PC_Systems.WBP Dialogue Cinematic` PlayerController) _returnvalue_2))))))

(event `End Text`
  (params (PlayerController :type "/Game/_GameManager/PC_Systems Object Reference"))
  (`/Game/UI/Menus/InGameMenu/WBP_Dialogue_Cinematic.CollapsedDialogueBox` (`/Game/_GameManager/PC_Systems.WBP Dialogue Cinematic` PlayerController)))

(event `Force End`
  (params (PlayerController :type "/Game/_GameManager/PC_Systems Object Reference"))
  (`/Game/UI/Menus/InGameMenu/WBP_EndScreen.ShowEndScreen` (`/Game/_GameManager/PC_Systems.WBP End Screen` PlayerController)))

(fn `Update`)