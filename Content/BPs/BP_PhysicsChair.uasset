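; Physics chair prop that players can kick, push or vacuum, with impulses driving its bottom mesh.
; A kick briefly flags it; hitting another kickable prop then breaks it, scoring points, spawning a separate bottom actor and destroying itself.
; Hits on other non-player actors send damage.
; Bound feedback events play sounds and feed Data Table positions, radii and mesh bounds into Niagara arrays for the debris burst.
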(event `self.ReceiveBeginPlay`
  (`self.Init Feedback`)
  (`PrimitiveComponent.AddImpulse` (`self.Bottom_Chair`) (0.0 0.0 2.0) "None" true))

(event `KickedInterface.Kicked`
  (params (KickVector :type "Vector Structure") (PlayerPosition :type "Vector Structure"))
  ;[0 0.4043 1 0.5] What happend when the chair got kicked
  (`self.Kicked_Sound_Event`)
  (set `self.IsKicked` true)
  (`KismetArrayLibrary.Array_Add` (`self.Tags`) "Kicked")
  (if (not (`self.IsBroken`))
    (`ActorComponent.Activate` (`self.VFX_Hit`) true)
    (`PrimitiveComponent.AddTorqueInDegrees` (`self.Top_Chair`) (0.0 0.0 50000.0) "None" true)
    (`PrimitiveComponent.AddImpulse` (`self.Bottom_Chair`) (* KickVector (`self.Impulse_Value`)) "None" false)
    (`KismetSystemLibrary.Delay` 1.0)
    (set `self.IsKicked` false)
    (`KismetArrayLibrary.Array_RemoveItem` (`self.Tags`) "Kicked")))

(event `self.ReceiveHit`
  (params (MyComp :type "PrimitiveComponent Object Reference") (Other :type "Actor Object Reference") (OtherComp :type "PrimitiveComponent Object Reference") (bSelfMoved :type Boolean) (HitLocation :type "Vector Structure") (HitNormal :type "Vector Structure") (NormalImpulse :type "Vector Structure") (Hit :type "HitResult Structure (by ref)"))
  (bind _top_chair (`self.Top_Chair`))
  (bind _vfx_hit (`self.VFX_Hit`))
  (bind _chair (`self.Chair`))
  (bind _returnvalue (`self.K2_GetActorLocation` (`.HitActor` (`GameplayStatics.BreakHitResult` Hit))))
  ;[1 0.51 0 0.5] Chair hit "Prop Physics" and what happend
  (`/Engine/EditorBlueprintResources/StandardMacros.IsValid` (`self.GetComponentByClass` Other "/Game/CppSystems/Prop/Public/ActorComponent/BP_Prop_PhysicsKickableCompBase_AC.BP_Prop_PhysicsKickableCompBase_AC_C")
    (:`Is Valid`
      (if (`self.IsKicked`)
        (`|ExecutionSequence`
          (:`then_0`
            (`SceneComponent.SetHiddenInGame` _top_chair true false)
            (`PrimitiveComponent.SetCollisionEnabled` _top_chair "NoCollision")
            (`KismetSystemLibrary.Delay` 0.1)
            (`PrimitiveComponent.SetCollisionResponseToChannel` (`self.Bottom_Chair`) "ECC_Pawn" "ECR_Ignore")
            (`PrimitiveComponent.SetSimulatePhysics` (`self.Bottom_Chair`) false)
            (`PrimitiveComponent.SetCollisionEnabled` (`self.Bottom_Chair`) "NoCollision")
            (`ActorComponent.Deactivate` (`self.Hitbox`))
            (set `self.IsBroken` true)
            (set `self.Chair` (`SceneComponent.K2_GetComponentToWorld` (`self.Bottom_Chair`)))
            (bind _bottom_chair (`self.Bottom_Chair`)
              (:`then`
                (`ActorComponent.K2_DestroyComponent` _bottom_chair)
                (`KismetSystemLibrary.DelayUntilNextTick`)
                (bind _returnvalue_2 (`|SpawnActorFromClass` "/Game/BPs/VacuumProps/BP_ChairBottom_Medium.BP_ChairBottom_Medium_C" (`KismetMathLibrary.MakeTransform` (`KismetMathLibrary.MakeVector` (.x (.location _chair)) (.y (.location _chair)) (+ (.z (.location _chair)) 5.0)) (.rotation _chair) (.scale _chair)) "AlwaysSpawn" "MultiplyWithRoot" null null null))
                (`KismetSystemLibrary.Delay` 0.15)
                (`PrimitiveComponent.SetSimulatePhysics` (`/Game/BPs/VacuumProps/BP_SuckableProp.StaticMesh` _returnvalue_2) true)
                (`KismetSystemLibrary.DelayUntilNextTick`)
                (`ActorComponent.K2_DestroyComponent` (`self.Hitbox`))
                (`KismetSystemLibrary.Delay` 2.0)
                (`self.K2_DestroyActor`))
              (:`else`)))
          (:`then_1`
            (`SceneComponent.K2_SetWorldLocation` _vfx_hit _returnvalue false false)
            (`SceneComponent.K2_SetWorldLocation` (`self.VFX_Explosion`) _returnvalue false false)
            (set `self.Hit_Actor_Location` _returnvalue)
            (`self.Explode_Sound_Event`)
            (`ActorComponent.Activate` _vfx_hit true)
            (`self.Break_VFX`)
            (`/Engine/EditorBlueprintResources/StandardMacros.DoOnce` false
              (:`Completed`
                (`FTJ_ScoringSystem_Score.IncreaseWithText` (subsystem `/Game/CppSystems/ScoringSystem/Public/Blueprint/BP_ScoringSystem_Score`) 10 1 (`|FormatText` "Broke Chair")))))
          (:`then_2`
            (`KismetSystemLibrary.Delay` 0.2)
            (set `self.IsKicked` false)))))
    (:`Is Not Valid`
      (if (not (`self.ActorHasTag` Other "Player"))
        (message `HitInterface.GetHit` Other (`self.Hit_Damage`) 0.0 (0.0 0.0 0.0) 0.0 self)))))

(event `/Game/BPs/BPI_Push.Push`
  (params (Force :type "Vector Structure"))
  (`PrimitiveComponent.AddImpulse` (`self.Bottom_Chair`) Force "None" true))

(event `/Game/BPs/TestProps/BPI_VacuumReaction.ReactToVacuum`
  (params (Force :type "Vector Structure"))
  (`PrimitiveComponent.AddImpulse` (`self.Bottom_Chair`) (* Force (`self.Vacuum_Effect_Force`)) "None" true))

(event `Init Feedback`
  (`|ExecutionSequence`
    (:`then_0`
      (add `self.Kicked_Sound` (delegate `Kicked_Sound_Event`)))
    (:`then_1`
      (add `self.Explode_Sound` (delegate `Explode_Sound_Event`)))
    (:`then_3`
      (add `self.Break_VFX` (delegate `Break_VFX_Event`)))))

(event `Kicked_Sound_Event`
  ;[0 1 1 0.5] FB - Sound When Kicked
  (`GameplayStatics.SpawnSoundAtLocation` (`self.Sound_Chair_Kicked`) (`SceneComponent.K2_GetComponentLocation` (`self.Bottom_Chair`)) (struct) 1.0 1.0 0.0 null null))

(event `Explode_Sound_Event`
  ;[0 1 1 0.5] FB - Sound When Chair Explode
  (`GameplayStatics.SpawnSoundAtLocation` (`self.Sound_Chair_Explode`) (`self.Hit_Actor_Location`) (struct) 1.0 1.0 0.0 null null))

(event `Getting_Vaccumed_Event`)

(event `Break_VFX_Event`
  (bind _dt_positions (`self.DT_Positions`))
  (bind _ns (`self.NS`))
  (set `self.NS` (`self.VFX_Explosion`))
  (bind _outrownames (`DataTableFunctionLibrary.GetDataTableRowNames` _dt_positions))
  (for _array_element _outrownames
    (bind _returnvalue (`|GetDataTableRow` _dt_positions _array_element)
      (:`then`
        (bind (_position _radius) (break `/Game/VFX/DataTables/S_FX_GetVectorPositionOffsets` _returnvalue))
        (`KismetArrayLibrary.Array_AddUnique` (`self.Array Position`) _position)
        (`KismetArrayLibrary.Array_AddUnique` (`self.Array Radius`) _radius))))
  (`|ExecutionSequence`
    (:`then_0`
      (for _array_element_2 (`self.Array Mesh Renderer`)
        (bind (_returnvalue_origin _returnvalue_boxextent) (`KismetMathLibrary.BreakBoxSphereBounds` (`StaticMesh.GetBounds` (`.Mesh` (break `NiagaraMeshRendererMeshPropertiesBase` _array_element_2)))))
        (`KismetArrayLibrary.Array_AddUnique` (`self.Array Bounds`) (* _returnvalue_boxextent 2.0))))
    (:`then_1`
      (`NiagaraDataInterfaceArrayFunctionLibrary.SetNiagaraArrayPosition` _ns "Position_Array" (`self.Array Position`))
      (`NiagaraDataInterfaceArrayMesh.SetNiagaraArrayMesh` _ns "Mesh Array" (`self.Array Mesh Renderer`))
      (`NiagaraComponent.SetVariableMaterial` _ns "Material Interface" "/Game/Environment/Office/Materials/MI_ChairAB_00.MI_ChairAB_00")
      (`NiagaraDataInterfaceArrayFunctionLibrary.SetNiagaraArrayFloat` _ns "Mesh_Radius" (`self.Array Radius`))
      (`NiagaraDataInterfaceArrayFunctionLibrary.SetNiagaraArrayVector` _ns "Mesh_Dimensions" (`self.Array Bounds`))
      (`ActorComponent.Activate` _ns false))))

(fn `UserConstructionScript`
  (`StaticMeshComponent.SetStaticMesh` (`self.Top_Chair`) (`self.New Mesh Top`))
  (`StaticMeshComponent.SetStaticMesh` (`self.Bottom_Chair`) (`self.New Mesh Bottom`)))