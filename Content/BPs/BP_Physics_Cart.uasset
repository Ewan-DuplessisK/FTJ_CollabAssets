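; Physics-driven cart prop that can be kicked, pushed or pulled by a vacuum effect, and damages non-player pawns it hits.
; The construction script selects food or platter cart style, setting mesh, wheel positions and hitbox.
; Each reaction applies a mesh impulse; kicks also trigger VFX, sound and a temporary "Kicked" flag and tag.
; Tick yaws the four wheels from velocity direction, like swivel casters, while moving.
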(event `self.ReceiveTick`
  (params (DeltaSeconds :type "Float (single-precision)"))
  (bind _returnvalue (`self.GetVelocity`))
  (if (> (`KismetMathLibrary.VSize` _returnvalue) 10.0)
    (`SceneComponent.K2_SetRelativeRotation` (`self.Wheel_1`) (`KismetMathLibrary.MakeRotator` 0.0 0.0 (+ (.yaw (`KismetMathLibrary.MakeRotFromX` (`KismetMathLibrary.Normal` _returnvalue))) 90.0)) false false)
    (`SceneComponent.K2_SetRelativeRotation` (`self.Wheel_2`) (`KismetMathLibrary.MakeRotator` 0.0 0.0 (+ (.yaw (`KismetMathLibrary.MakeRotFromX` (`KismetMathLibrary.Normal` _returnvalue))) 90.0)) false false)
    (`SceneComponent.K2_SetRelativeRotation` (`self.Wheel_3`) (`KismetMathLibrary.MakeRotator` 0.0 0.0 (+ (.yaw (`KismetMathLibrary.MakeRotFromX` (`KismetMathLibrary.Normal` _returnvalue))) 90.0)) false false)
    (`SceneComponent.K2_SetRelativeRotation` (`self.Wheel_4`) (`KismetMathLibrary.MakeRotator` 0.0 0.0 (+ (.yaw (`KismetMathLibrary.MakeRotFromX` (`KismetMathLibrary.Normal` _returnvalue))) 90.0)) false false)))

(event `self.ReceiveBeginPlay`
  (`self.Init Feedback`)
  (`PrimitiveComponent.AddImpulse` (`self.Mesh`) (0.0 0.0 2.0) "None" true))

(event `self.Kicked`
  (params (KickVector :type "Vector Structure") (PlayerPosition :type "Vector Structure"))
  ;[0 0.4043 1 0.5] What happend when the chair got kicked
  (`self.Kicked_Sound_Event`)
  (set `self.IsKicked` true)
  (`KismetArrayLibrary.Array_Add` (`self.Tags`) "Kicked")
  (`ActorComponent.Activate` (`self.VFX_Hit`) true)
  (`PrimitiveComponent.AddImpulse` (`self.Mesh`) (* KickVector (`self.Impulse_Value`)) "None" false)
  (`KismetSystemLibrary.Delay` 1.0)
  (set `self.IsKicked` false)
  (`KismetArrayLibrary.Array_RemoveItem` (`self.Tags`) "Kicked"))

(event `self.ReceiveHit`
  (params (MyComp :type "PrimitiveComponent Object Reference") (Other :type "Actor Object Reference") (OtherComp :type "PrimitiveComponent Object Reference") (bSelfMoved :type Boolean) (HitLocation :type "Vector Structure") (HitNormal :type "Vector Structure") (NormalImpulse :type "Vector Structure") (Hit :type "HitResult Structure (by ref)"))
  ;[1 0.51 0 0.5] Chair hit "Prop Physics" and what happend
  (if (not (`self.ActorHasTag` Other "Player"))
    (bind _aspawn (cast `Pawn` Other))
    (message `HitInterface.GetHit` _aspawn (`self.Damage`) 0.0 (0.0 0.0 0.0) (`self.Invincibility Time`) null)))

(event `self.Push`
  (params (Force :type "Vector Structure"))
  (`PrimitiveComponent.AddImpulse` (`self.Mesh`) Force "None" true))

(event `self.ReactToVacuum`
  (params (Force :type "Vector Structure"))
  (`PrimitiveComponent.AddImpulse` (`self.Mesh`) (* Force (`self.Vacuum_Effect_Force`)) "None" true))

(event `Init Feedback`
  (`|ExecutionSequence`
    (:`then_0`
      (add `self.Kicked_Sound` (delegate `Kicked_Sound_Event`)))))

(event `Kicked_Sound_Event`
  ;[0 1 1 0.5] FB - Sound When Kicked
  (`GameplayStatics.SpawnSoundAtLocation` (`self.Sound_Chair_Kicked`) (`SceneComponent.K2_GetComponentLocation` (`self.Mesh`)) (struct) 1.0 1.0 0.0 null null))

(fn `UserConstructionScript`
  (bind _hitbox (`self.Hitbox`))
  (switch `/Game/BPs/Enums/E_Cart` (`self.Cart Style`)
    (:`NewEnumerator0`
      (`StaticMeshComponent.SetStaticMesh` (`self.Mesh`) "/Game/Environment/Office/Meshes/Furniture/Carts/FoodCart/SM_FoodCart_01.SM_FoodCart_01")
      (`self.Wheel Position` (28.0 23.0 18.0) (-29.0 23.0 18.0) (-33.0 -23.0 18.0) (33.0 -23.0 18.0))
      (`BoxComponent.SetBoxExtent` _hitbox (45.0 45.0 50.0) true)
      (`SceneComponent.K2_SetRelativeLocation` _hitbox (0.0 0.0 59.0) false false))
    (:`NewEnumerator1`
      (`StaticMeshComponent.SetStaticMesh` (`self.Mesh`) "/Game/Environment/Office/Meshes/Furniture/Carts/PlatterCart/SM_PlatterCart_01.SM_PlatterCart_01")
      (`self.Wheel Position` (48.0 22.0 9.0) (-20.0 22.0 9.0) (-20.0 -31.0 9.0) (48.0 -31.0 9.0))
      (`BoxComponent.SetBoxExtent` _hitbox (40.0 40.0 95.0) true)
      (`SceneComponent.K2_SetRelativeLocation` _hitbox (14.0 -2.0 93.0) false false))))

(fn `Wheel Position`
  (params (`Wheel 1` :type "Vector Structure") (`Wheel 2` :type "Vector Structure") (`Wheel 3` :type "Vector Structure") (`Wheel 4` :type "Vector Structure"))
  (`|ExecutionSequence`
    (:`then_0`
      (`SceneComponent.K2_SetRelativeLocation` (`self.Wheel_1`) `Wheel 1` false false))
    (:`then_1`
      (`SceneComponent.K2_SetRelativeLocation` (`self.Wheel_2`) `Wheel 2` false false))
    (:`then_2`
      (`SceneComponent.K2_SetRelativeLocation` (`self.Wheel_3`) `Wheel 3` false false))
    (:`then_3`
      (`SceneComponent.K2_SetRelativeLocation` (`self.Wheel_4`) `Wheel 4` false false))))