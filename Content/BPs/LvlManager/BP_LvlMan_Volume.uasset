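; BP_LvlMan_Volume is a trigger box paired with a level streaming volume, recording the player's first walk through it.
; SetVolume fits the box to the volume's bounds.
; On first overlap, or overlap shortly after BeginPlay, it scales the volume to MAXV3 and notifies BP_LvlMan.
; Load, unload and reload events toggle the volume's scale between MAXV3 and zero, with blocking stream calls for its first level.
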(event `self.ReceiveBeginPlay`
  (`KismetSystemLibrary.Delay` 2.0)
  (if (`PrimitiveComponent.IsOverlappingActor` (`self.Box`) (`GameplayStatics.GetPlayerPawn` 0))
    (if (not (`self.Walked`)) :!label _label
      (`KismetSystemLibrary.Delay` 0.1)
      (`self.SetActorScale3D` (`self.Volume`) (`self.MAX_V3`))
      (set `self.Walked` true)
      (`/Game/BPs/LvlManager/BP_LvlMan.Set Volume WalkedThrough` (`self.Get LvlMan`) self))))

(event `self.ReceiveActorBeginOverlap`
  (params (OtherActor :type "Actor Object Reference"))
  (`self.Is Player` OtherActor
    (:`true`
      (goto _label))))

(event `self.Box.OnComponentBeginOverlap`
  (params (OverlappedComponent :type "PrimitiveComponent Object Reference") (OtherActor :type "Actor Object Reference") (OtherComp :type "PrimitiveComponent Object Reference") (OtherBodyIndex :type Integer) (bFromSweep :type Boolean) (SweepResult :type "HitResult Structure (by ref)"))
  (`self.Is Player` OverlappedComponent
    (:`true`
      (goto _label))))

(event `Set Volume`
  (params (Volume :type "LevelStreamingVolume Object Reference"))
  (bind _box (`self.Box`))
  (bind (_origin _boxextent) (`KismetSystemLibrary.GetComponentBounds` (`Brush.BrushComponent` (`self.Volume`))))
  (set `self.Volume` Volume)
  (`BoxComponent.SetBoxExtent` _box _boxextent true)
  (`SceneComponent.K2_SetWorldLocation` _box _origin false true))

(event `Unload Level`
  (bind _volume (`self.Volume`))
  (`self.SetActorScale3D` _volume (0.0 0.0 0.0))
  (`GameplayStatics.UnloadStreamLevel` (`|GetArrayItem` (`LevelStreamingVolume.StreamingLevelNames` _volume)) true)
  (`GameplayStatics.FlushLevelStreaming`))

(event `Load Level`
  (bind _volume (`self.Volume`))
  (`self.SetActorScale3D` _volume (`self.MAX_V3`))
  (`GameplayStatics.LoadStreamLevel` (`|GetArrayItem` (`LevelStreamingVolume.StreamingLevelNames` _volume)) true true)
  (`GameplayStatics.FlushLevelStreaming`))

(event `Reload Level`
  (`self.Unload Level`)
  (`KismetSystemLibrary.Delay` 0.2)
  (`self.Load Level`))

(fn `Get LvlMan`
  (returns (ReturnValue :type "/Game/BPs/LvlManager/BP_LvlMan Object Reference"))
  (bind _returnvalue (`GameplayStatics.GetActorOfClass` "/Game/BPs/LvlManager/BP_LvlMan.BP_LvlMan_C"))
  (return _returnvalue))

(fn `UserConstructionScript`)