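; BP_LvlMan is the level manager, handling streamed-level volumes and checkpoint respawns.
; At BeginPlay it spawns a BP_LvlMan_Volume per LevelStreamingVolume, mapped by level name and source volume, and starts an 8000-second timed quit.
; Respawn moves the player, reloads the checkpoint's volume and reapplies checkpoint data, or restarts the level if there is no checkpoint or a full-reload level is set.
; It also records walked-through volumes and has a test reload event.
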(event `self.ReceiveBeginPlay`
  (`|ExecutionSequence`
    (:`then_0`
      (bind _returnvalue (`GameplayStatics.GetActorOfClass` "/Game/Characters/Player/Blueprints/BP_Player.BP_Player_C"))
      (set `self.Player` _returnvalue))
    (:`then_1`
      (bind _outactors (`GameplayStatics.GetAllActorsOfClass` "/Script/Engine.LevelStreamingVolume"))
      (bind _output_get (set `self.LevelVolumes` _outactors))
      (for _array_element _output_get
        (bind (_returnvalue_location _returnvalue_rotation) (`KismetMathLibrary.BreakTransform` (`self.GetTransform` _array_element)))
        (bind _returnvalue_2 (`|SpawnActorFromClass` "/Game/BPs/LvlManager/BP_LvlMan_Volume.BP_LvlMan_Volume_C" (`KismetMathLibrary.MakeTransform` _returnvalue_location _returnvalue_rotation) "Undefined" "MultiplyWithRoot" null null))
        (`/Game/BPs/LvlManager/BP_LvlMan_Volume.Set Volume` _returnvalue_2 _array_element)
        (`|ExecutionSequence`
          (:`then_0`
            (bind (_lefts _rights) (`KismetStringLibrary.Split` (`KismetStringLibrary.Conv_NameToString` (`|GetArrayItem` (`LevelStreamingVolume.StreamingLevelNames` (`/Game/BPs/LvlManager/BP_LvlMan_Volume.Volume` _returnvalue_2)))) "_0_" "IgnoreCase" "FromEnd"))
            (`BlueprintMapLibrary.Map_Add` (`self.LvlVolume By LevelName`) (`KismetStringLibrary.Conv_StringToName` _rights) _returnvalue_2)
            (`KismetSystemLibrary.PrintString` _rights true true (struct :`G` 0.66 :`B` 1.0 :`A` 1.0) 1000.0 :!enabledstate Disabled))
          (:`then_1`
            (`BlueprintMapLibrary.Map_Add` (`self.LvlVolume By LevelVolume`) _array_element _returnvalue_2)))))
    (:`then_2`
      (`KismetSystemLibrary.Delay` 8000.0)
      (`KismetSystemLibrary.QuitGame` null "Quit"))))

(event `Respawn from Current Checkpoint`
  (bind _current_checkpoint (`self.Current Checkpoint`))
  (`/Game/Characters/Player/Blueprints/BP_Player.ShowLoading` (`self.Player`))
  (`GameplayStatics.SetGamePaused` true)
  (`/Engine/EditorBlueprintResources/StandardMacros.IsValid` _current_checkpoint
    (:`Is Valid`
      (if (`KismetSystemLibrary.IsValidSoftObjectReference` (`/Game/BPs/LvlManager/BP_LvlMan_Checkpoint.Full Reload Level` _current_checkpoint))
        (`/Game/Developers/vladislavpavlov/LevelManager/GI_Systems_Base.Restart Level` (`/Game/Characters/Player/Blueprints/WeaponSystem/Interactable/FL_Common.Get GI Systems`) :!label _label)
        (else
          (`/Game/Characters/Player/Blueprints/BP_Player.Set Transform` (`self.Player`) (`self.GetTransform` (`self.Current Checkpoint`)))
          (`/Game/BPs/LvlManager/BP_LvlMan_Volume.Reload Level` (`BlueprintMapLibrary.Map_Find` (`self.LvlVolume By LevelVolume`) (`/Game/BPs/LvlManager/BP_LvlMan_Checkpoint.Level Volume` (`self.Current Checkpoint`))))
          (`/Game/BPs/LvlManager/BP_LvlMan_Checkpoint.Apply Checkpoint Data` (`self.Current Checkpoint`))
          (`/Game/Characters/Player/Blueprints/BP_Player.Enable Playing` (`self.Player`))
          (`GameplayStatics.SetGamePaused` false))))
    (:`Is Not Valid`
      (goto _label))))

(event `Set Volume WalkedThrough`
  (params (NewItem :type "/Game/BPs/LvlManager/BP_LvlMan_Volume Object Reference (by ref)"))
  (bind _returnvalue (`KismetArrayLibrary.Array_AddUnique` (`self.WalkedThrough`) NewItem))
  (`KismetSystemLibrary.PrintString` (`KismetStringLibrary.Concat_StrStr` "Volume Walked: index - " (`KismetStringLibrary.Conv_IntToString` _returnvalue))))

(event `TEST Reaload 01`
  (bind (_value _returnvalue) (`BlueprintMapLibrary.Map_Find` (`self.LvlVolume By LevelName`) "LVL_01"))
  ; TEST reload
  (bind _outactors (`GameplayStatics.GetAllActorsOfClass` "/Script/Engine.PlayerStart"))
  (`self.K2_SetActorTransform` (`GameplayStatics.GetPlayerPawn` 0) (`self.GetTransform` (`|GetArrayItem` _outactors)) false true)
  (if _returnvalue
    (`/Game/BPs/LvlManager/BP_LvlMan_Volume.Unload Level` _value)
    (`KismetSystemLibrary.Delay` 1.0)
    (`/Game/BPs/LvlManager/BP_LvlMan_Volume.Load Level` _value)
    (else
      (`KismetSystemLibrary.PrintString` "[LevelManager]: Level not found"))))

(fn `Set Current Checkpoint`
  (params (`Current Checkpoint` :type "/Game/BPs/LvlManager/BP_LvlMan_Checkpoint Object Reference"))
  (returns (Changed :type Boolean))
  (locals (_Changed :type Boolean))
  (bind _output_get (set `local._Changed` (!= (`self.Current Checkpoint`) `Current Checkpoint`)))
  (if _output_get
    (set `self.Current Checkpoint` `Current Checkpoint`))
  (return _output_get))

(fn `UserConstructionScript`)