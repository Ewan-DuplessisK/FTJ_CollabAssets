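; Level checkpoint actor that snapshots and restores player progress for BP_LvlMan.
; Player overlap with its Triggers actors, or its own collision when none are set (rechecked shortly after BeginPlay), activates it once.
; If the level manager accepts it as current, it saves score, BP_Player health and serialized BP_Vacuum inventory.
; ApplyCheckpointData writes that snapshot back and resets the score multiplier to one.
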(event `Bind Trigger`
  (`|ExecutionSequence`
    (:`then_1`
      (add `self.OnActorBeginOverlap` (stale `self.ReceiveBeginPlay` _array_element) (delegate `OnActorBeginOverlap_Event`) :!label _label))))

(event `OnActorBeginOverlap_Event` :!signature `self.OnActorBeginOverlap`
  (params (OverlappedActor :type "Actor Object Reference") (OtherActor :type "Actor Object Reference"))
  (`self.on Overlap` OtherActor))

(event `self.ReceiveBeginPlay`
  (bind _returnvalue (`GameplayStatics.GetPlayerPawn` 0))
  (bind _triggers (`self.Triggers`))
  (if (`KismetArrayLibrary.Array_IsNotEmpty` _triggers)
    (for _array_element _triggers
      (goto _label))
    (else
      (add `PrimitiveComponent.OnComponentBeginOverlap` (`self.CollisionComponent`) (delegate `OnComponentBeginOverlap_Event`))
      (`KismetSystemLibrary.Delay` 0.2)
      (if (`PrimitiveComponent.IsOverlappingActor` (`self.CollisionComponent`) _returnvalue)
        (`self.on Overlap` _returnvalue)))))

(event `OnComponentBeginOverlap_Event`
  (params (OverlappedComponent :type "PrimitiveComponent Object Reference") (OtherActor :type "Actor Object Reference") (OtherComp :type "PrimitiveComponent Object Reference") (OtherBodyIndex :type Integer) (bFromSweep :type Boolean) (SweepResult :type "HitResult Structure (by ref)"))
  (`self.on Overlap` OtherActor))

(event `Set as Current`
  (if (not (`self.Walked`))
    (set `self.Walked` true)
    (bind _changed (`/Game/BPs/LvlManager/BP_LvlMan.Set Current Checkpoint` (`self.Get LvlMan`) self))
    (if _changed
      (`self.Save Checkpoint Data`))))

(fn `Apply Checkpoint Data`
  (bind _returnvalue (subsystem `/Game/CppSystems/ScoringSystem/Public/Blueprint/BP_ScoringSystem_Score`))
  (bind (_saved_scores _saved_hp _saved_ammo) (break `/Game/BPs/LvlManager/F_LvlMan_Checkpoint_Save2` (`self.Saved`)))
  (bind _returnvalue_2 (`KismetMathLibrary.FTrunc` _saved_scores))
  (`KismetSystemLibrary.PrintString` (`KismetStringLibrary.Concat_StrStr` (`KismetStringLibrary.Conv_IntToString` _returnvalue_2) "  HP: " (`KismetStringLibrary.Conv_DoubleToString` _saved_hp)))
  (bind _returnvalue_3 (`GameplayStatics.GetActorOfClass` "/Game/Characters/Player/Blueprints/BP_Player.BP_Player_C"))
  (`FTJ_ScoringSystem_ScoreBase.SetScore` _returnvalue _returnvalue_2)
  (`FTJ_ScoringSystem_ScoreBase.SetMultiplier` _returnvalue 1)
  (`HealthInterface.AddHealth` _returnvalue_3 _saved_hp)
  (set `FTJ_CharaBase.CurrentHealth` _saved_hp _returnvalue_3)
  (bind _returnvalue_4 (`GameplayStatics.GetActorOfClass` "/Game/Characters/Player/Blueprints/BP_Vacuum.BP_Vacuum_C"))
  (`/Game/Characters/Player/Blueprints/BP_Vacuum.Set Inventory Serialized` _returnvalue_4 _saved_ammo)
  (`KismetSystemLibrary.PrintText` (`|FormatText` "[LvlMan_Checkpoint]: Save HP={hp}, Score={score}" _saved_hp _returnvalue_2)))

(fn `Get LvlMan`
  (returns (ReturnValue :type "/Game/BPs/LvlManager/BP_LvlMan Object Reference"))
  (bind _returnvalue (`GameplayStatics.GetActorOfClass` "/Game/BPs/LvlManager/BP_LvlMan.BP_LvlMan_C"))
  (return _returnvalue))

(fn `on Overlap`
  (params (A :type "Object Object Reference"))
  (if (== A (`GameplayStatics.GetPlayerPawn` 0))
    (`self.Set as Current`)))

(fn `Save Checkpoint Data`
  (bind _returnvalue (`KismetMathLibrary.Conv_IntToDouble` (`FTJ_ScoringSystem_ScoreBase.GetScore` (subsystem `/Game/CppSystems/ScoringSystem/Public/Blueprint/BP_ScoringSystem_Score`))))
  (bind _returnvalue_2 (`GameplayStatics.GetActorOfClass` "/Game/Characters/Player/Blueprints/BP_Player.BP_Player_C"))
  (bind _returnvalue_3 (`GameplayStatics.GetActorOfClass` "/Game/Characters/Player/Blueprints/BP_Vacuum.BP_Vacuum_C"))
  (bind _inventoryclasses (`/Game/Characters/Player/Blueprints/BP_Vacuum.Get Inventory Serialized` _returnvalue_3))
  (bind _currenthealth (`FTJ_CharaBase.CurrentHealth` _returnvalue_2))
  (set `self.Saved` (make `/Game/BPs/LvlManager/F_LvlMan_Checkpoint_Save2` _returnvalue _currenthealth _inventoryclasses))
  (`KismetSystemLibrary.PrintText` (`|FormatText` "[LvlMan_Checkpoint]: Save HP={hp}, Score={score}" _currenthealth _returnvalue)))

(fn `UserConstructionScript`)