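; BP_Arena_Door is an arena door that slides vertically between closed and open positions.
; On BeginPlay it stores the Cube's relative location as closed and derives the open position from its Z scale plus a movement buffer.
; OpenDoor and CloseDoor set the DoorOpen flag and play or reverse a timeline, which lerps the Cube's Z between the two positions.
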(event `self.ReceiveBeginPlay`
  (bind _cube (`self.Cube`))
  (bind (_relativescale3d_x _relativescale3d_y _relativescale3d_z) (`KismetMathLibrary.BreakVector` (`SceneComponent.RelativeScale3D` _cube)))
  (bind _output_get (set `self.Closed Position` (`SceneComponent.RelativeLocation` _cube)))
  (set `self.Open Position` (`KismetMathLibrary.MakeVector` (.x _output_get) (.y _output_get) (+ (.z _output_get) (* _relativescale3d_z (+ 100.0 (`self.Door Movement Buffer`)))))))

(event `Open Door`
  (bind _cube (`self.Cube`))
  (bind (_open_position_x _open_position_y _open_position_z) (`KismetMathLibrary.BreakVector` (`self.Open Position`)))
  (bind (_closed_position_x _closed_position_y _closed_position_z) (`KismetMathLibrary.BreakVector` (`self.Closed Position`)))
  (bind (_relativelocation_x _relativelocation_y) (`KismetMathLibrary.BreakVector` (`SceneComponent.RelativeLocation` _cube)))
  (set `self.Door Open` true)
  (bind (_direction _alpha) (`Timeline|T_Door Swing` :!label _label)
    (:`Update`
      (`SceneComponent.K2_SetRelativeLocation` _cube (`KismetMathLibrary.MakeVector` _relativelocation_x _relativelocation_y (`KismetMathLibrary.Lerp` _closed_position_z _open_position_z _alpha)) false false))))

(event `Close Door`
  (set `self.Door Open` false)
  (goto _label :!via `Reverse`))

(fn `UserConstructionScript`)