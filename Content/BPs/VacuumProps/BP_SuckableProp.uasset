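; BP_SuckableProp is a physics prop that can be stored in an inventory and launched back into the world as a damaging projectile.
; Storing shrinks it and disables tick, physics and collision; placing or pushing re-enables them, re-arms damage and briefly shows a trail.
; A DoOnce limits each launch to one damaging hit on non-player actors.
; Each hit costs durability; at zero the prop awards score and destroys itself.
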(event `self.ReceiveBeginPlay`)

(event `Add to Inventory`
  (params (Location :type "Vector Structure"))
  (`self.SetActorTickEnabled` false)
  (`PrimitiveComponent.SetSimulatePhysics` (`self.StaticMesh`) false)
  (`self.K2_SetActorTransform` (`KismetMathLibrary.MakeTransform` Location (struct) (0.01 0.01 0.01)))
  (`PrimitiveComponent.SetCollisionEnabled` (`self.StaticMesh`) "NoCollision"))

(event `Place to World`
  (params (Location :type "Vector Structure") (Rotation :type "Rotator Structure"))
  (`self.K2_SetActorTransform` (`KismetMathLibrary.MakeTransform` Location Rotation))
  (`self.SetActorTickEnabled` true)
  (`PrimitiveComponent.SetSimulatePhysics` (`self.StaticMesh`) true)
  (`PrimitiveComponent.SetCollisionEnabled` (`self.StaticMesh`) "QueryAndPhysics")
  (`self.ResetHit`)
  (`self.ActivateTrail`))

(event `self.ReceiveHit`
  (params (MyComp :type "PrimitiveComponent Object Reference") (Other :type "Actor Object Reference") (OtherComp :type "PrimitiveComponent Object Reference") (bSelfMoved :type Boolean) (HitLocation :type "Vector Structure") (HitNormal :type "Vector Structure") (NormalImpulse :type "Vector Structure") (Hit :type "HitResult Structure (by ref)"))
  (`|ExecutionSequence`
    (:`then_0`
      (`self.On Suckable Hit`))
    (:`then_1`
      (if (and (`self.DamageEnabled`) (not (`self.ActorHasTag` Other "Player")))
        (`/Engine/EditorBlueprintResources/StandardMacros.DoOnce` false :!label _label
          (:`Completed`
            (message `HitInterface.GetHit` Other (`self.Damage`) 0.0 (0.0 0.0 0.0) 0.0 null)
            (message `HealthInterface.DamageBreakable` Other (`self.DamageToBreakable`) HitNormal)
            (`|ExecutionSequence`
              (:`then_0`
                (`KismetSystemLibrary.Delay` 0.1)
                (set `self.DamageEnabled` false))
              (:`then_1`
                (`self.LooseDurability`)))))))))

(event `ResetHit`
  (set `self.DamageEnabled` true)
  (goto _label :!via `Reset`))

(event `ActivateTrail`
  (bind _trail (`self.Trail`))
  (`ActorComponent.Activate` _trail true)
  (`KismetSystemLibrary.Delay` 3.0)
  (`ActorComponent.Deactivate` _trail))

(event `LooseDurability`
  (bind _result (`/Engine/EditorBlueprintResources/StandardMacros.DecrementInt` (`self.Health`))
    (:`  `
      (if (<= _result 0)
        (`FTJ_ScoringSystem_Score.IncreaseWithText` (subsystem `/Game/CppSystems/ScoringSystem/Public/Blueprint/BP_ScoringSystem_Score`) (`self.ScoreOnDestruction`) (`self.MultiplierOnDestruction`) (`self.MessageOnDestruction`))
        (`KismetSystemLibrary.DelayUntilNextTick`)
        (`self.K2_DestroyActor`)))))

(event `/Game/BPs/BPI_Push.Push`
  (params (Force :type "Vector Structure"))
  (`self.Place to World` (`self.K2_GetActorLocation`) (`self.K2_GetActorRotation`))
  (`PrimitiveComponent.AddImpulse` (`self.StaticMesh`) Force "None" false))

(event `self.ReceiveEndPlay`
  (params (EndPlayReason :type "EEndPlayReason Enum" :default "Destroyed"))
  (`self.K2_DestroyActor`))

(event `Init Feedback`
  (`|ExecutionSequence`
    (:`then_0`
      (add `self.On Suckable Hit` (delegate `On Suckable Hit_Event`)))))

(event `On Suckable Hit_Event`)

(fn `UserConstructionScript`
  (`StaticMeshComponent.SetStaticMesh` (`self.StaticMesh`) (`self.Mesh`)))