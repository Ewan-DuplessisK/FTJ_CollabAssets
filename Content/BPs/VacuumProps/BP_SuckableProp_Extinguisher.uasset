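; Suckable fire extinguisher prop that, when active and hitting something other than the player or another suckable prop, flies erratically before exploding.
; A looping timer applies leak thrust and random torque with a foam trail, and hits damage non-player pawns.
; After the flight duration, a timeline deforms the material.
; Sphere traces then damage and knock back pawns, push props and damage breakables before the actor destroys itself.
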(event `self.ReceiveHit`
  (params (MyComp :type "PrimitiveComponent Object Reference") (Other :type "Actor Object Reference") (OtherComp :type "PrimitiveComponent Object Reference") (bSelfMoved :type Boolean) (HitLocation :type "Vector Structure") (HitNormal :type "Vector Structure") (NormalImpulse :type "Vector Structure") (Hit :type "HitResult Structure (by ref)"))
  (cast `/Game/BPs/VacuumProps/BP_SuckableProp` Other
    (:`CastFailed`
      (bind _aspawn (cast `Pawn` Other)
        (:`then`
          (if (not (`self.ActorHasTag` _aspawn "Player"))
            (message `HitInterface.GetHit` _aspawn (`self.DamageWhenFlying`) 0.0 (0.0 0.0 0.0) 0.0 null)
            (if (`self.IsActive`) :!label _label
              (`/Engine/EditorBlueprintResources/StandardMacros.DoOnce` false
                (:`Completed`
                  (bind _returnvalue (`KismetSystemLibrary.K2_SetTimerDelegate` (delegate `ExtinguisherFly`) 0.033333 true true))
                  (set `self.FlightTimeHandle` _returnvalue))))))
        (:`CastFailed`
          (goto _label))))))

(event `ExtinguisherFly`
  (`PrimitiveComponent.AddForce` (`self.StaticMesh`) (* (* (`SceneComponent.GetUpVector` (`self.StaticMesh`)) (`KismetMathLibrary.Conv_DoubleToVector` -1.0)) (`self.Leaking_Speed`)) "None" true)
  (`PrimitiveComponent.AddTorqueInDegrees` (`self.StaticMesh`) (* (`KismetMathLibrary.RandomUnitVector`) (`self.RandomDirectionForce`)) "None" true)
  (`/Engine/EditorBlueprintResources/StandardMacros.DoOnce` false
    (:`Completed`
      (bind _returnvalue (`KismetSystemLibrary.K2_SetTimerDelegate` (delegate `Explode`) 0.03 false false (`self.FlightDuration`)))
      (set `self.ExplosionTimeHandle` _returnvalue)
      (`NiagaraComponent.SetAsset` (`self.Trail`) "/Game/VFX/Niagara/Props/Extinguisher/NS_Foam_Extinguisher.NS_Foam_Extinguisher" true))))

(event `Explode`
  (bind _returnvalue (`self.K2_GetActorLocation`))
  (bind _returnvalue_2 (`self.K2_GetActorLocation`))
  (bind _returnvalue_3 (`self.K2_GetActorLocation`))
  (bind _staticmesh (`self.StaticMesh`))
  (`KismetSystemLibrary.K2_ClearAndInvalidateTimerHandle` (`self.FlightTimeHandle`))
  (`KismetSystemLibrary.DelayUntilNextTick`)
  (bind _returnvalue_4 (`PrimitiveComponent.CreateDynamicMaterialInstance` (`self.StaticMesh`) 0 null "None"))
  (set `self.DynMatRef` _returnvalue_4)
  (bind (_direction _explosion) (`Timeline|Timeline` :!via `PlayFromStart`)
    (:`Update`
      (`/Engine/EditorBlueprintResources/StandardMacros.IsValid` (`self.StaticMesh`)
        (:`Is Valid`
          (`MaterialInstanceDynamic.SetScalarParameterValue` (`self.DynMatRef`) "Positions_Boing" _explosion))))
    (:`Finished`
      (`PrimitiveComponent.SetSimulatePhysics` _staticmesh false)
      (`PrimitiveComponent.SetCollisionEnabled` _staticmesh "NoCollision")
      (`SceneComponent.SetHiddenInGame` (`self.StaticMesh`) false false)
      (`ActorComponent.Activate` (`self.NS_Explosion`) false)
      (bind _outhits (`KismetSystemLibrary.SphereTraceMultiForObjects` :`Start` _returnvalue_3 :`End` _returnvalue_3 :`Radius` (`self.AOE_Radius`) :`ObjectTypes` (`|MakeArray` "ObjectTypeQuery3" "ObjectTypeQuery19" :!type "EObjectTypeQuery Enum") :`DrawDebugType` "ForDuration"))
      (for _array_element _outhits
        (bind (_bblockinghit _binitialoverlap _time _distance _location _impactpoint _normal _impactnormal _physmat _hitactor) (`GameplayStatics.BreakHitResult` _array_element))
        (message `HitInterface.GetHit` _hitactor (`self.Damage`) 0.0 (* (- (`self.K2_GetActorLocation` _hitactor) (`self.K2_GetActorLocation`)) (`self.PushForceEnemies`)) 0.0 null))
      (bind _outhits_2 (`KismetSystemLibrary.SphereTraceMultiForObjects` :`Start` _returnvalue_2 :`End` _returnvalue_2 :`Radius` (`self.AOE_Radius`) :`ObjectTypes` (`|MakeArray` "ObjectTypeQuery13" :!type "EObjectTypeQuery Enum") :`DrawDebugType` "ForDuration"))
      (for _array_element_2 _outhits_2
        (bind (_bblockinghit_2 _binitialoverlap_2 _time_2 _distance_2 _location_2 _impactpoint_2 _normal_2 _impactnormal_2 _physmat_2 _hitactor_2) (`GameplayStatics.BreakHitResult` _array_element_2))
        (message `/Game/BPs/BPI_Push.Push` _hitactor_2 (* (- (`self.K2_GetActorLocation` _hitactor_2) (`self.K2_GetActorLocation`)) (`self.PushForceProps`))))
      (bind _outhits_3 (`KismetSystemLibrary.SphereTraceMultiForObjects` :`Start` _returnvalue :`End` _returnvalue :`Radius` (`self.AOE_Radius`) :`ObjectTypes` (`|MakeArray` "ObjectTypeQuery4" "ObjectTypeQuery2" :!type "EObjectTypeQuery Enum") :`DrawDebugType` "ForDuration"))
      (for _array_element_3 _outhits_3
        (message `HealthInterface.DamageBreakable` (`.HitActor` (`GameplayStatics.BreakHitResult` _array_element_3)) (`self.DamageToBreakable`) (`KismetMathLibrary.Normal` (- (`self.K2_GetActorLocation`) (`self.K2_GetActorLocation`)))))
      (`KismetSystemLibrary.Delay` 0.2)
      (`self.K2_DestroyActor`))))

(fn `UserConstructionScript`
  (`parent.UserConstructionScript`))