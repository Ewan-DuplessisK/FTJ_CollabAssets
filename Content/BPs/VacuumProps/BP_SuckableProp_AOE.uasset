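; Area-of-effect variant of a suckable vacuum prop that explodes when it hits anything other than another suckable prop while active.
; Three debug-drawn sphere traces send messages to damage and knock back pawns, push props, and damage breakables.
; Knockback and prop push scale with unnormalized distance from the blast, while the breakable push subtracts the actor's own location, giving zero.
; It then plays the explosion effect, hides and disables its mesh, and destroys itself after a delay.
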(event `self.ReceiveHit`
  (params (MyComp :type "PrimitiveComponent Object Reference") (Other :type "Actor Object Reference") (OtherComp :type "PrimitiveComponent Object Reference") (bSelfMoved :type Boolean) (HitLocation :type "Vector Structure") (HitNormal :type "Vector Structure") (NormalImpulse :type "Vector Structure") (Hit :type "HitResult Structure (by ref)"))
  (bind _returnvalue (`self.K2_GetActorLocation`))
  (bind _returnvalue_2 (`self.K2_GetActorLocation`))
  (bind _returnvalue_3 (`self.K2_GetActorLocation`))
  (bind _staticmesh (`self.StaticMesh`))
  (cast `/Game/BPs/VacuumProps/BP_SuckableProp` Other
    (:`CastFailed`
      (if (`self.IsActive`)
        (bind _outhits (`KismetSystemLibrary.SphereTraceMultiForObjects` :`Start` _returnvalue_3 :`End` _returnvalue_3 :`Radius` (`self.AOE_Radius`) :`ObjectTypes` (`|MakeArray` "ObjectTypeQuery3" "ObjectTypeQuery19" :!type "EObjectTypeQuery Enum") :`DrawDebugType` "ForDuration"))
        (for _array_element _outhits
          (bind (_bblockinghit _binitialoverlap _time _distance _location _impactpoint _normal _impactnormal _physmat _hitactor) (`GameplayStatics.BreakHitResult` _array_element))
          (message `HitInterface.GetHit` _hitactor (`self.Damage`) 0.0 (* (- (`self.K2_GetActorLocation` _hitactor) (`self.K2_GetActorLocation`)) (`self.PushForceEnemies`)) 0.0 null))
        (bind _outhits_2 (`KismetSystemLibrary.SphereTraceMultiForObjects` :`Start` _returnvalue_2 :`End` _returnvalue_2 :`Radius` (`self.AOE_Radius`) :`ObjectTypes` (`|MakeArray` "ObjectTypeQuery13" :!type "EObjectTypeQuery Enum") :`DrawDebugType` "ForDuration"))
        (for _array_element_2 _outhits_2
          (bind (_bblockinghit_2 _binitialoverlap_2 _time_2 _distance_2 _location_2 _impactpoint_2 _normal_2 _impactnormal_2 _physmat_2 _hitactor_2) (`GameplayStatics.BreakHitResult` _array_element_2))
          (message `/Game/BPs/BPI_Push.Push` _hitactor_2 (* (- (`self.K2_GetActorLocation` _hitactor_2) (`self.K2_GetActorLocation`)) (`self.PushForceProps`))))
        (bind _outhits_3 (`KismetSystemLibrary.SphereTraceMultiForObjects` :`Start` _returnvalue :`End` _returnvalue :`Radius` (`self.AOE_Radius`) :`ObjectTypes` (`|MakeArray` "ObjectTypeQuery4" "ObjectTypeQuery2" :!type "EObjectTypeQuery Enum") :`DrawDebugType` "ForDuration"))
        (for _array_element_3 _outhits_3
          (message `HealthInterface.DamageBreakable` (`.HitActor` (`GameplayStatics.BreakHitResult` _array_element_3)) (`self.DamageToBreakable`) (`KismetMathLibrary.Normal` (- (`self.K2_GetActorLocation`) (`self.K2_GetActorLocation`)))))
        (`ActorComponent.Activate` (`self.NS_Explosion`) false)
        (`SceneComponent.SetHiddenInGame` _staticmesh true false)
        (`PrimitiveComponent.SetCollisionEnabled` _staticmesh "NoCollision")
        (`KismetSystemLibrary.Delay` 5.0)
        (`self.K2_DestroyActor`)))))

(fn `UserConstructionScript`
  (`parent.UserConstructionScript`))