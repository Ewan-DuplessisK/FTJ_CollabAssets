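; Elevator actor that acts as a locked exit, opened through a DoorOpen event.
; DoorOpen hides the Cube door, disables its collision and has the Progress object play the elevator-unlocked dialogue on the player controller.
; When the player pawn overlaps the Inside trigger while IsOpen is true, it calls ForceEnd on Progress; IsOpen is not set in these graphs.
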(event `self.ReceiveBeginPlay`
  (bind _asgi_systems (cast `/Game/_GameManager/GI_Systems` (`GameplayStatics.GetGameInstance`)))
  (set `self.As GI Systems` _asgi_systems))

(event `Door Open`
  (bind _cube (`self.Cube`))
  (`SceneComponent.SetHiddenInGame` _cube true false)
  (`PrimitiveComponent.SetCollisionEnabled` _cube "NoCollision")
  (bind _aspc_systems (cast `/Game/_GameManager/PC_Systems` (`GameplayStatics.GetPlayerController` 0)))
  (`/Game/Progress/Blueprint/BP_Progress_Progress.Dialogue` (subsystem `/Game/Progress/Blueprint/BP_Progress_Progress`) _aspc_systems "D_Elevator_Unlocked" false))

(event `self.Inside.OnComponentBeginOverlap`
  (params (OverlappedComponent :type "PrimitiveComponent Object Reference") (OtherActor :type "Actor Object Reference") (OtherComp :type "PrimitiveComponent Object Reference") (OtherBodyIndex :type Integer) (bFromSweep :type Boolean) (SweepResult :type "HitResult Structure (by ref)"))
  (if (and (`self.Is Open`) (== OtherActor (`GameplayStatics.GetPlayerPawn` 0)))
    (bind _aspc_systems (cast `/Game/_GameManager/PC_Systems` (`GameplayStatics.GetPlayerController` 0)))
    (`/Game/Progress/Blueprint/BP_Progress_Progress.Force End` (subsystem `/Game/Progress/Blueprint/BP_Progress_Progress`) _aspc_systems)))

(fn `UserConstructionScript`)