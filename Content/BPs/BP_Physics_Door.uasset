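; Breakable physics door that shatters when kicked, rammed or reduced to zero health, with optional debug HP text.
; Fast Heavy actors, other doors and kicked chairs trigger Kicked from Hit, while GetHit applies damage with timed invincibility.
; Kicked launches the mesh, then swaps it once for a BP_Door_Test Geometry Collection that receives the same impulse.
; Kick and break sounds play through bound events; the despawn logic is unconnected.
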(event `self.ReceiveBeginPlay`
  (bind _hp_render (`self.Hp Render`))
  (`self.Init Feedback`)
  (set `self.CurrentHealth` (`self.MaxHealth`))
  (`self.Set HP Visual`)
  (if (`self.Debug_Health_Show`)
    (`SceneComponent.SetVisibility` _hp_render true false)
    (`SceneComponent.SetVisibility` (`self.Hp Render1`) true false)
    (else
      (`SceneComponent.SetVisibility` _hp_render false false)
      (`SceneComponent.SetVisibility` (`self.Hp Render1`) false false))))

(event `KickedInterface.Kicked`
  (params (KickVector :type "Vector Structure") (PlayerPosition :type "Vector Structure"))
  (bind _staticmesh (`self.StaticMesh`))
  ;[0 0.4075 1 0.5] What happens when you kick the door
  (`PrimitiveComponent.SetSimulatePhysics` (`self.StaticMesh`) true)
  (set `self.IsKicked` true)
  (bind _output_get (set `self.Kick Strength` (* KickVector (`self.Impulse Strength`))))
  (`PrimitiveComponent.AddImpulse` (`self.StaticMesh`) _output_get "None" true)
  (`self.Kicked_Sound_Event`)
  ;[0.15 0 0 0.5] Event Hit
  (`/Engine/EditorBlueprintResources/StandardMacros.DoOnce` false
    (:`Completed`
      (bind _returnvalue (`self.Spawn Window Breakable` (`SceneComponent.K2_GetComponentLocation` _staticmesh) (`SceneComponent.K2_GetComponentRotation` _staticmesh)))
      (bind _output_get_2 (set `self.Fractured_Door` _returnvalue))
      (`|ExecutionSequence`
        (:`then_0`
          ;;[0.561 0 0.6979 0.5] Door Spawn & Explosion when hit something
          (`PrimitiveComponent.AddImpulse` (`/Game/BPs/GC_GCBP/test/BP_Door_Test.GeometryCollection` _output_get_2) (/ (`self.Kick Strength`) 1.0) "None" true)
          (`ActorComponent.K2_DestroyComponent` (`self.StaticMesh`))
          (`ActorComponent.K2_DestroyComponent` (`self.Box`))
          (`self.Break_Sound_Event`))
        (:`then_1`)))))

(event `self.ReceiveHit`
  (params (MyComp :type "PrimitiveComponent Object Reference") (Other :type "Actor Object Reference") (OtherComp :type "PrimitiveComponent Object Reference") (bSelfMoved :type Boolean) (HitLocation :type "Vector Structure") (HitNormal :type "Vector Structure") (NormalImpulse :type "Vector Structure") (Hit :type "HitResult Structure (by ref)"))
  (bind (_returnvalue_roll _returnvalue_pitch _returnvalue_yaw) (`KismetMathLibrary.BreakRotator` (`self.K2_GetActorRotation`)))
  (bind _returnvalue (* (`self.GetVelocity` Other) (`self.GetActorRightVector`)))
  ;[0.15 0 0 0.5] Event Hit
  (if (> (`KismetMathLibrary.VSize` (`self.GetVelocity` Other)) (`self.Velocity Threshold`))
    (if (or (`self.ActorHasTag` Other "Heavy") (`KismetStringLibrary.Contains` (`KismetSystemLibrary.GetDisplayName` Other) "Door") (and (`self.ActorHasTag` Other "Chair") (`self.ActorHasTag` Other "Kicked")))
      (if (!= _returnvalue_yaw -90.0)
        (`KickedInterface.Kicked` (* _returnvalue 10.0))
        (else
          (`KickedInterface.Kicked` (* _returnvalue -10.0)))))))

(event `HealthInterface.DamageBreakable`
  (params (Damage :type "Float (single-precision)") (Push :type "Vector Structure"))
  (bind _output_get (set `self.CurrentHealth` (`KismetMathLibrary.FClamp` (- (`self.CurrentHealth`) Damage) 0.0 (`self.MaxHealth`))))
  (`self.Set HP Visual`)
  (if (<= _output_get 0.0)
    (`/Engine/EditorBlueprintResources/StandardMacros.DoOnce` false
      (:`Completed`
        (`KickedInterface.Kicked` (stale `HitInterface.GetHit` KnockbackVector))))))

(event `HitInterface.GetHit`
  (params (Damage :type "Float (single-precision)") (HitStunDuration :type "Float (single-precision)") (KnockbackVector :type "Vector Structure") (InvincibilityTime :type "Float (single-precision)") (SourceActor :type "Actor Object Reference"))
  ;[1 0.2455 0.000893 0.5 50] GetHit
  (if (not (`self.IsInvincible`))
    (`|ExecutionSequence`
      (:`then_0`
        (`HealthInterface.DamageBreakable` Damage)
        (set `self.IsInvincible` true)
        (bind _returnvalue (`KismetSystemLibrary.K2_SetTimer` null "InvinsibilityReset" (`KismetMathLibrary.FMax` InvincibilityTime 0.01) false true))
        (set `self.InvinsibilityTimer` _returnvalue))
      (:`then_1`))))

(event `Set HP Visual`
  (`TextRenderComponent.K2_SetText` (`self.Hp Render`) (`KismetTextLibrary.Conv_DoubleToText` (`self.CurrentHealth`) "HalfToEven"))
  (`TextRenderComponent.K2_SetText` (`self.Hp Render1`) (`KismetTextLibrary.Conv_DoubleToText` (`self.CurrentHealth`) "HalfToEven")))

(event `Init Feedback`
  (`|ExecutionSequence`
    (:`then_0`
      (add `self.Kicked_Sound` (delegate `Kicked_Sound_Event`)))
    (:`then_1`
      (add `self.Break_Sound` (delegate `Break_Sound_Event`)))))

(event `Kicked_Sound_Event`
  (`GameplayStatics.PlaySoundAtLocation` (`self.Sound_When_Kicked`) (`SceneComponent.K2_GetComponentLocation` (`self.StaticMesh`)) (struct) 1.0 1.0 0.0 null null null null))

(event `Break_Sound_Event`
  ;[0 1 1 0.5] FB - Sound When Break
  (`GameplayStatics.PlaySoundAtLocation` (`self.Sound_When_Break`) (`self.K2_GetActorLocation` (`self.Fractured_Door`)) (struct) 1.0 1.0 0.0 null null null null))

(fn `Spawn Window Breakable`
  (params (SpawnTransform_Location :type "Vector Structure") (`Spawn Transform Rotation` :type "Rotator Structure"))
  (returns (ReturnValue :type "/Game/BPs/GC_GCBP/test/BP_Door_Test Object Reference"))
  (bind _returnvalue (`|SpawnActorFromClass` "/Game/BPs/GC_GCBP/test/BP_Door_Test.BP_Door_Test_C" (`KismetMathLibrary.MakeTransform` SpawnTransform_Location `Spawn Transform Rotation`) "AlwaysSpawn" "MultiplyWithRoot" null null))
  (return _returnvalue))

(fn `UserConstructionScript`
  (bind _hp_render (`self.Hp Render`))
  (set `self.CurrentHealth` (`self.MaxHealth`))
  (`self.Set HP Visual`)
  (if (`self.Debug_Health_Show`)
    (`SceneComponent.SetVisibility` _hp_render true false)
    (`SceneComponent.SetVisibility` (`self.Hp Render1`) true false)
    (else
      (`SceneComponent.SetVisibility` _hp_render false false)
      (`SceneComponent.SetVisibility` (`self.Hp Render1`) false false))))