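; BP_Spawner is a placeable spawner that creates an instance of a configurable actor class on demand.
; The construction script sizes its Sphere component from SpawnSphereRadius.
; SpawnActor places the actor one radius above the sphere's center with the sphere's rotation and a configurable scale, adjusting for collisions but always spawning.
; It returns the new actor, or prints an error when the class is invalid.
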(fn `Spawn Actor`
  (returns (`Out Actor` :type "Actor Object Reference"))
  (bind _sphere (`self.Sphere`))
  (bind _actor_to_spawn (`self.Actor to Spawn`))
  (bind (_returnvalue_location _returnvalue_rotation) (`KismetMathLibrary.BreakTransform` (`SceneComponent.K2_GetComponentToWorld` _sphere)))
  (if (`KismetSystemLibrary.IsValidClass` _actor_to_spawn)
    (bind _returnvalue (`|SpawnActorFromClass` _actor_to_spawn (`KismetMathLibrary.MakeTransform` (+ _returnvalue_location (`KismetMathLibrary.MakeVector` 0.0 0.0 (`SphereComponent.SphereRadius` _sphere))) _returnvalue_rotation (`self.Spawn Actor Scale`)) "AdjustIfPossibleButAlwaysSpawn" "MultiplyWithRoot" null null))
    (return _returnvalue)
    (else
      (`KismetSystemLibrary.PrintString` "Invalid Class to spawn in BP_Spawn"))))

(fn `UserConstructionScript`
  (`SphereComponent.SetSphereRadius` (`self.Sphere`) (`self.Spawn Sphere Radius`) true))