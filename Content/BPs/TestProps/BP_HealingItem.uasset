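; BP_HealingItem is a pickup that heals the player when they touch it.
; On collision sphere overlap with the BP_Player pawn, it checks for missing health, or allows pickup at full health when PickupIfFullHealth is set.
; It then passes HealingValue to AddHealthMessage, waits a tick, plays the heal sound and destroys itself.
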(event `self.Collision_Sphere.OnComponentBeginOverlap`
  (params (OverlappedComponent :type "PrimitiveComponent Object Reference") (OtherActor :type "Actor Object Reference") (OtherComp :type "PrimitiveComponent Object Reference") (OtherBodyIndex :type Integer) (bFromSweep :type Boolean) (SweepResult :type "HitResult Structure (by ref)"))
  (bind _asbp_player (cast `/Game/Characters/Player/Blueprints/BP_Player` (`GameplayStatics.GetPlayerCharacter` 0) :!pure true))
  (if (== OtherActor _asbp_player)
    (if (< (`FTJ_CharaBase.CurrentHealth` _asbp_player) (`FTJ_CharaBase.MaxHealth` _asbp_player))
      (message `HealthInterface.AddHealth` _asbp_player (`self.Healing_Value`) :!label _label)
      (`KismetSystemLibrary.DelayUntilNextTick`)
      (`GameplayStatics.PlaySound2D` "/Game/_GameManager/Feedbacks/Sounds/Heal/SC_Snak_Heal_Cue.SC_Snak_Heal_Cue" 1.0 1.0 0.0 null null)
      (`self.K2_DestroyActor`)
      (elif (`self.Pickup If Full Health`)
        (goto _label)))))

(fn `UserConstructionScript`)