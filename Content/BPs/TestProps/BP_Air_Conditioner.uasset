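; BP_Air_Conditioner is a breakable air conditioner prop that awards score when struck.
; A Box overlap by an actor tagged Heavy, Medium or Light marks it broken, fires the OnHit dispatcher and disables Box collision.
; The Feedback graph binds OnHit at BeginPlay to play sound and scaled VFX, activate two spark effects and raise score and multiplier with an "AirCo" message.
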(event `self.ReceiveBeginPlay`
  (`self.Init Feedback`))

(event `self.Box.OnComponentBeginOverlap`
  (params (OverlappedComponent :type "PrimitiveComponent Object Reference") (OtherActor :type "Actor Object Reference") (OtherComp :type "PrimitiveComponent Object Reference") (OtherBodyIndex :type Integer) (bFromSweep :type Boolean) (SweepResult :type "HitResult Structure (by ref)"))
  (if (or (`self.ActorHasTag` OtherActor "Heavy") (`self.ActorHasTag` OtherActor "Medium") (`self.ActorHasTag` OtherActor "Light"))
    (set `self.Is Broken` true)
    (`self.On Hit`)
    (`PrimitiveComponent.SetCollisionEnabled` (`self.Box`) "NoCollision")))

(event `Init Feedback`
  (`|ExecutionSequence`
    (:`then_0`
      (add `self.On Hit` (delegate `On Hit_Event`)))))

(event `On Hit_Event`
  (bind _staticmesh (`self.StaticMesh`))
  ;[0 1 1 0.5] Sound When Hit
  (`GameplayStatics.SpawnSoundAtLocation` (`self.Sound When Hit`) (`SceneComponent.K2_GetComponentLocation` (`self.StaticMesh`)) (struct) 1.0 1.0 0.0 null null)
  ;[0 1 1] VFX
  (`NiagaraFunctionLibrary.SpawnSystemAtLocation` (`self.VFX When Hit`) (+ (`SceneComponent.K2_GetComponentLocation` _staticmesh) (0.0 -20.0 50.0)) (`SceneComponent.K2_GetComponentRotation` _staticmesh) (/ (`self.GetActorScale3D`) 5.0))
  (`ActorComponent.Activate` (`self.NS_Burst_Spark_Loop`) false)
  (`ActorComponent.Activate` (`self.NS_Burst_Spark_Loop1`) false)
  (`FTJ_ScoringSystem_Score.IncreaseWithText` (subsystem `/Game/CppSystems/ScoringSystem/Public/Blueprint/BP_ScoringSystem_Score`) 15 1 (`|FormatText` "Broke AirCo")))

(fn `UserConstructionScript`)