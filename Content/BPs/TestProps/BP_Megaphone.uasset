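; Breakable megaphone prop with four animated speaker meshes that awards player score when broken.
; A looping timer, started once Animate is true, or CallAnimation plays a timeline driving material parameters, recreating dynamic instances every update.
; CallAnimation also activates speaking Niagara effects, which deactivate when the timeline finishes or is stopped.
; Overlap by Heavy, Medium or Light tagged actors disables box collision and fires OnHit for sound, VFX and score.
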(event `self.ReceiveBeginPlay`
  (`self.Init Feedback`))

(event `self.ReceiveTick`
  (params (DeltaSeconds :type "Float (single-precision)"))
  (if (`self.Animate`)
    (`/Engine/EditorBlueprintResources/StandardMacros.DoOnce` false
      (:`Completed`
        (`KismetSystemLibrary.K2_SetTimerDelegate` (delegate `Megaphone Loop`) 5.0 true true)))))

(event `self.Box.OnComponentBeginOverlap`
  (params (OverlappedComponent :type "PrimitiveComponent Object Reference") (OtherActor :type "Actor Object Reference") (OtherComp :type "PrimitiveComponent Object Reference") (OtherBodyIndex :type Integer) (bFromSweep :type Boolean) (SweepResult :type "HitResult Structure (by ref)"))
  (if (or (`self.ActorHasTag` OtherActor "Heavy") (`self.ActorHasTag` OtherActor "Medium") (`self.ActorHasTag` OtherActor "Light"))
    (set `self.Is Broken` true)
    (`self.On Hit`)
    (`PrimitiveComponent.SetCollisionEnabled` (`self.Box`) "NoCollision")))

(event `Megaphone Loop`
  (bind _sm_megaphone_a_01 (`self.SM_Megaphone_A_01`))
  (bind _sm_megaphone_b_01 (`self.SM_Megaphone_B_01`))
  (bind _sm_megaphone_c_01 (`self.SM_Megaphone_C_01`))
  (bind _sm_megaphone_d_01 (`self.SM_Megaphone_D_01`))
  (bind (_direction _newtrack_0) (`Timeline|TL_Speakers` :!via `PlayFromStart` :!label _label)
    (:`Update`
      (`|ExecutionSequence`
        (:`then_0`
          (bind _returnvalue (`PrimitiveComponent.CreateDynamicMaterialInstance` _sm_megaphone_a_01 0 (`PrimitiveComponent.GetMaterial` _sm_megaphone_a_01 0) "None"))
          (`MaterialInstanceDynamic.SetScalarParameterValue` _returnvalue "Animation_VC" _newtrack_0)
          (bind _returnvalue_2 (`MaterialInstanceDynamic.K2_GetScalarParameterValue` _returnvalue "Time"))
          (`MaterialInstanceDynamic.SetScalarParameterValue` _returnvalue "PrevTime" _returnvalue_2)
          (`MaterialInstanceDynamic.SetScalarParameterValue` _returnvalue "Time" _newtrack_0))
        (:`then_1`
          (bind _returnvalue_3 (`PrimitiveComponent.CreateDynamicMaterialInstance` _sm_megaphone_b_01 0 (`PrimitiveComponent.GetMaterial` _sm_megaphone_b_01 0) "None"))
          (`MaterialInstanceDynamic.SetScalarParameterValue` _returnvalue_3 "Animation_VC" _newtrack_0)
          (bind _returnvalue_4 (`MaterialInstanceDynamic.K2_GetScalarParameterValue` _returnvalue_3 "Time"))
          (`MaterialInstanceDynamic.SetScalarParameterValue` _returnvalue_3 "PrevTime" _returnvalue_4)
          (`MaterialInstanceDynamic.SetScalarParameterValue` _returnvalue_3 "Time" _newtrack_0))
        (:`then_2`
          (bind _returnvalue_5 (`PrimitiveComponent.CreateDynamicMaterialInstance` _sm_megaphone_c_01 0 (`PrimitiveComponent.GetMaterial` _sm_megaphone_c_01 0) "None"))
          (`MaterialInstanceDynamic.SetScalarParameterValue` _returnvalue_5 "Animation_VC" _newtrack_0)
          (bind _returnvalue_6 (`MaterialInstanceDynamic.K2_GetScalarParameterValue` _returnvalue_5 "Time"))
          (`MaterialInstanceDynamic.SetScalarParameterValue` _returnvalue_5 "PrevTime" _returnvalue_6)
          (`MaterialInstanceDynamic.SetScalarParameterValue` _returnvalue_5 "Time" _newtrack_0))
        (:`then_3`
          (bind _returnvalue_7 (`PrimitiveComponent.CreateDynamicMaterialInstance` _sm_megaphone_d_01 0 (`PrimitiveComponent.GetMaterial` _sm_megaphone_d_01 0) "None"))
          (`MaterialInstanceDynamic.SetScalarParameterValue` _returnvalue_7 "Animation_VC" _newtrack_0)
          (bind _returnvalue_8 (`MaterialInstanceDynamic.K2_GetScalarParameterValue` _returnvalue_7 "Time"))
          (`MaterialInstanceDynamic.SetScalarParameterValue` _returnvalue_7 "PrevTime" _returnvalue_8)
          (`MaterialInstanceDynamic.SetScalarParameterValue` _returnvalue_7 "Time" _newtrack_0))))
    (:`Finished`
      (`ActorComponent.Deactivate` (`self.NS_Megaphone_Speak3`) :!label _label_2)
      (`ActorComponent.Deactivate` (`self.NS_Megaphone_Speak2`))
      (`ActorComponent.Deactivate` (`self.NS_Megaphone_Speak1`))
      (`ActorComponent.Deactivate` (`self.NS_Megaphone_Speak`)))))

(event `/Game/BPs/TestProps/BPI/BPI_Megaphone.Call Animation`
  (params (`Is True` :type Boolean))
  (if `Is True`
    (`ActorComponent.Activate` (`self.NS_Megaphone_Speak3`) false)
    (`ActorComponent.Activate` (`self.NS_Megaphone_Speak2`) false)
    (`ActorComponent.Activate` (`self.NS_Megaphone_Speak1`) false)
    (`ActorComponent.Activate` (`self.NS_Megaphone_Speak`) false)
    (goto _label :!via `PlayFromStart`)
    (else
      (`|ExecutionSequence`
        (:`then_0`
          (goto _label :!via `Stop`))
        (:`then_1`
          (goto _label_2))))))

(event `Init Feedback`
  (`|ExecutionSequence`
    (:`then_0`
      (add `self.On Hit` (delegate `On Hit_Event`)))))

(event `On Hit_Event`
  (bind _returnvalue (- (`SceneComponent.K2_GetComponentLocation` (`self.StaticMesh`)) (0.0 0.0 30.0)))
  ;[0 1 1 0.5] Sound When Hit
  (`GameplayStatics.SpawnSoundAtLocation` (`self.Sound When Hit`) _returnvalue (struct) 1.0 1.0 0.0 null null)
  ;[0 1 1] VFX
  (`NiagaraFunctionLibrary.SpawnSystemAtLocation` (`self.VFX When Hit`) _returnvalue (`SceneComponent.K2_GetComponentRotation` (`self.StaticMesh`)) (/ (`self.GetActorScale3D`) 10.0))
  (`FTJ_ScoringSystem_Score.IncreaseWithText` (`self.GetComponentByClass` (`GameplayStatics.GetPlayerCharacter` 0) "/Game/CppSystems/ScoringSystem/Public/ActorComponent/BP_ScoringSystem_Score_AC.BP_ScoringSystem_Score_AC_C") 10 1 (`|FormatText` "Broke Megaphone")))

(fn `UserConstructionScript`)