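; Player controller that routes Enhanced Input to the first-person player and vacuum (suck/blow, kick, look).
; BeginPlay loads camera feel from a data asset, creates timer and in-game menu widgets, disables pawn input, starts a countdown, and spawns a debug menu outside packaged builds.
; Sphere-trace lock-on supports sideways target switching and steers the camera on Tick, while a timeline drives 180-degree turns.
; Visualizer input actions feed an on-screen controller display.
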(event `EnhancedInput|/Game/_GameManager/Inputs/Actions/IA_Select`
  (params (ActionValue :type Boolean) (ElapsedSeconds :type "Float (double-precision)") (TriggeredSeconds :type "Float (double-precision)") (InputAction :type "InputAction Object Reference" :default "/Game/_GameManager/Inputs/Actions/IA_Select.IA_Select"))
  (:`Triggered`
    (`GameplayStatics.OpenLevelBySoftObjectPtr` "/Game/Developers/thomasabate/L_Gym_Thomas.L_Gym_Thomas")))

(event `EnhancedInput|/Game/_GameManager/Inputs/Actions/IA_Kick`
  (params (ActionValue :type Boolean) (ElapsedSeconds :type "Float (double-precision)") (TriggeredSeconds :type "Float (double-precision)") (InputAction :type "InputAction Object Reference" :default "/Game/_GameManager/Inputs/Actions/IA_Kick.IA_Kick"))
  ;[0 0 0 0.4 75] IA Kick
  (:`Started`
    (`/Game/Characters/Player/Blueprints/BP_Player.Kick` (`self.As BP Player`))))

(event `self.ReceiveBeginPlay`
  (bind _returnvalue (subsystem `EnhancedInputLocalPlayerSubsystem`))
  (bind _timer_widget (`self.Timer Widget`))
  ;[0 0 0 0.4 75] Begin play
  (`self.SetCameraFeel`)
  (`parent.ReceiveBeginPlay`)
  (`|ExecutionSequence`
    (:`then_0`
      (`EnhancedInputSubsystemInterface.AddMappingContext` _returnvalue "/Game/_GameManager/Inputs/IMC_FThisJob.IMC_FThisJob" 0 (struct))
      (bind _asgi_systems (cast `/Game/_GameManager/GI_Systems` (`GameplayStatics.GetGameInstance`))
        (:`then`
          (set `self.GI_Systems` _asgi_systems)
          ;;[1 0.05865 0.00022 0.5 30] Timer
          (bind _returnvalue_2 (`|CreateWidget` "/Game/UI/WBP_Timer.WBP_Timer_C"))
          (set `self.Timer Widget` _returnvalue_2)
          (`UserWidget.AddToViewport` _timer_widget 0)
          (`Widget.SetVisibility` _timer_widget "Hidden")
          (bind _asbp_player (cast `/Game/Characters/Player/Blueprints/BP_Player` (`self.K2_GetPawn`)))
          (set `self.As BP Player` _asbp_player)
          (bind _asbp_vacuum (cast `/Game/Characters/Player/Blueprints/BP_Vacuum` (`ChildActorComponent.ChildActor` (`/Game/Characters/Player/Blueprints/BP_Player.Vacuum` (`self.As BP Player`)))))
          (set `self.As BP Vacuum` _asbp_vacuum))
        (:`CastFailed`
          (`KismetSystemLibrary.PrintString` "CAST GI_INSTANCE FAILED" true true (struct :`R` 1.0 :`B` 0.035124 :`A` 1.0) 50.0))))
    (:`then_1`
      (`EnhancedInputSubsystemInterface.AddMappingContext` _returnvalue "/Game/UI/Debug/ControllerInputVisualizer/Inputs/IMC_ControllerVisualizer.IMC_ControllerVisualizer" 1 (struct))
      (`self.DisableInput` (`self.As BP Player`) self))
    (:`then_2`
      (`self.Generate Widget`)
      (`/Game/UI/Menus/InGameMenu/WBP_BigNumber.StartCoutdownBegin` (`self.WBP Big Number`) 5.25))
    (:`then_3`
      (if (not (`KismetSystemLibrary.IsPackagedForDistribution`))
        (`|SpawnActorFromClass` "/Game/Developers/vladislavpavlov/Dbg/BP_Dbg_Menu.BP_Dbg_Menu_C" (`KismetMathLibrary.Conv_VectorToTransform` (`KismetMathLibrary.Vector_Zero`)) "Undefined" "MultiplyWithRoot" null self)))))

(event `EnhancedInput|/Game/_GameManager/Inputs/Actions/IA_Vacuum_Suck`
  (params (ActionValue :type Boolean) (ElapsedSeconds :type "Float (double-precision)") (TriggeredSeconds :type "Float (double-precision)") (InputAction :type "InputAction Object Reference" :default "/Game/_GameManager/Inputs/Actions/IA_Vacuum_Suck.IA_Vacuum_Suck"))
  ;[0 0 0 0.4 75] IA Vacuum
  ;;[0.15 0.15 0.15 0.5 50] Vacuum
  (:`Triggered`
    (`/Engine/EditorBlueprintResources/StandardMacros.Gate` true :!label _label
      (:`Exit`
        (`/Game/Characters/Player/Blueprints/BP_Vacuum.VacuumTick` (`self.As BP Vacuum`)))))
  (:`Started`
    (`|ExecutionSequence`
      (:`then_0`
        (goto _label :!via `Open`))
      (:`then_1`
        (`/Game/Characters/Player/Blueprints/BP_Vacuum.Start Sucking` (`self.As BP Vacuum`)))
      (:`then_2`
        (goto _label_3 :!via `Close`))))
  (:`Canceled`
    (`/Game/Characters/Player/Blueprints/BP_Vacuum.Stop Sucking` (`self.As BP Vacuum`) :!label _label_2))
  (:`Completed`
    (goto _label_2)))

(event `EnhancedInput|/Game/_GameManager/Inputs/Actions/IA_Vacuum_Shoot`
  (params (ActionValue :type Boolean) (ElapsedSeconds :type "Float (double-precision)") (TriggeredSeconds :type "Float (double-precision)") (InputAction :type "InputAction Object Reference" :default "/Game/_GameManager/Inputs/Actions/IA_Vacuum_Shoot.IA_Vacuum_Shoot"))
  ;[0 0 0 0.4 75] IA Vacuum
  ;;[0.15 0.15 0.15 0.5 50] Vacuum
  (:`Triggered`
    (`/Engine/EditorBlueprintResources/StandardMacros.Gate` true :!label _label_3
      (:`Exit`
        (`/Game/Characters/Player/Blueprints/BP_Vacuum.BlowTick` (`self.As BP Vacuum`)))))
  (:`Started`
    (`|ExecutionSequence`
      (:`then_0`
        (goto _label :!via `Close`))
      (:`then_1`
        (goto _label_3 :!via `Open`)))))

(event `self.ReceiveTick`
  (params (DeltaSeconds :type "Float (single-precision)"))
  (bind _returnvalue (`self.K2_GetActorRotation`))
  ;[0 0 0 0.4 75] EventTick
  (`|ExecutionSequence`
    (:`then_0`
      (`self.SendControllerVisualizerData`))
    (:`then_1`
      ;[0 0 0 0.4 75] Lock On
      ;;[0.9 0.8 0 1 50] Target Lock On
      (if (`self.TargetLocked`)
        (bind _lock_target_actor (`self.Lock Target Actor`)
          (:`then`
            (bind (_returnvalue_x _returnvalue_y _returnvalue_z) (`KismetMathLibrary.BreakVector` (`self.K2_GetActorLocation` _lock_target_actor)))
            (bind (_returnvalue_roll _returnvalue_pitch _returnvalue_yaw) (`KismetMathLibrary.BreakRotator` (`KismetMathLibrary.RInterpTo` _returnvalue (`KismetMathLibrary.FindLookAtRotation` (`self.K2_GetActorLocation` (`self.PlayerCharacterRef`)) (`KismetMathLibrary.MakeVector` _returnvalue_x _returnvalue_y (`KismetMathLibrary.FClamp` (- _returnvalue_z (`self.Max Close Distance Between Player / Ennemy`)) 50.0 125.0))) (`GameplayStatics.GetWorldDeltaSeconds`) 15.0)))
            (`self.SetControlRotation` (`KismetMathLibrary.MakeRotator` (.roll _returnvalue) _returnvalue_pitch _returnvalue_yaw))
            (if (or (>= (`self.GetDistanceTo` (`self.Lock Target Actor`) (`self.PlayerCharacterRef`)) (`self.Auto Unlock Distance`)) (`self.ActorHasTag` _lock_target_actor (`self.Tag Death`)))
              (set `self.Lock Target Actor` null)
              (set `self.TargetLocked` false)
              (set `self.LockOn Switch` false)))
          (:`else`))))))

(event `EnhancedInput|/Game/UI/Debug/ControllerInputVisualizer/Inputs/IA_Visu_DPad_Left`
  (params (ActionValue :type Boolean) (ElapsedSeconds :type "Float (double-precision)") (TriggeredSeconds :type "Float (double-precision)") (InputAction :type "InputAction Object Reference" :default "/Game/UI/Debug/ControllerInputVisualizer/Inputs/IA_Visu_DPad_Left.IA_Visu_DPad_Left"))
  ;[0 0 0 0.33 75] ControllerVisualizer Debug
  ;;[0.3557 1 0.4036 0.33] DPad
  (:`Started`
    (`/Game/UI/Debug/ControllerInputVisualizer/WBP_ControllerInputsVisualizer.ReceiveInputVisualizationData_Button` (`self.Controller Input Visualizer`) true "NewEnumerator1"))
  (:`Completed`
    (`/Game/UI/Debug/ControllerInputVisualizer/WBP_ControllerInputsVisualizer.ReceiveInputVisualizationData_Button` (`self.Controller Input Visualizer`) false "NewEnumerator1")))

(event `EnhancedInput|/Game/UI/Debug/ControllerInputVisualizer/Inputs/IA_Visu_DPad_Bottom`
  (params (ActionValue :type Boolean) (ElapsedSeconds :type "Float (double-precision)") (TriggeredSeconds :type "Float (double-precision)") (InputAction :type "InputAction Object Reference" :default "/Game/UI/Debug/ControllerInputVisualizer/Inputs/IA_Visu_DPad_Bottom.IA_Visu_DPad_Bottom"))
  ;[0 0 0 0.33 75] ControllerVisualizer Debug
  ;;[0.3557 1 0.4036 0.33] DPad
  (:`Started`
    (`/Game/UI/Debug/ControllerInputVisualizer/WBP_ControllerInputsVisualizer.ReceiveInputVisualizationData_Button` (`self.Controller Input Visualizer`) true "NewEnumerator0"))
  (:`Completed`
    (`/Game/UI/Debug/ControllerInputVisualizer/WBP_ControllerInputsVisualizer.ReceiveInputVisualizationData_Button` (`self.Controller Input Visualizer`) false "NewEnumerator0")))

(event `EnhancedInput|/Game/UI/Debug/ControllerInputVisualizer/Inputs/IA_Visu_FaceButton_Bottom`
  (params (ActionValue :type Boolean) (ElapsedSeconds :type "Float (double-precision)") (TriggeredSeconds :type "Float (double-precision)") (InputAction :type "InputAction Object Reference" :default "/Game/UI/Debug/ControllerInputVisualizer/Inputs/IA_Visu_FaceButton_Bottom.IA_Visu_FaceButton_Bottom"))
  ;[0 0 0 0.33 75] ControllerVisualizer Debug
  ;;[1 0.5477 0.8376 0.33] Face Button
  (:`Started`
    (`/Game/UI/Debug/ControllerInputVisualizer/WBP_ControllerInputsVisualizer.ReceiveInputVisualizationData_Button` (`self.Controller Input Visualizer`) true "NewEnumerator4"))
  (:`Completed`
    (`/Game/UI/Debug/ControllerInputVisualizer/WBP_ControllerInputsVisualizer.ReceiveInputVisualizationData_Button` (`self.Controller Input Visualizer`) false "NewEnumerator4")))

(event `EnhancedInput|/Game/UI/Debug/ControllerInputVisualizer/Inputs/IA_Visu_FaceButton_Left`
  (params (ActionValue :type Boolean) (ElapsedSeconds :type "Float (double-precision)") (TriggeredSeconds :type "Float (double-precision)") (InputAction :type "InputAction Object Reference" :default "/Game/UI/Debug/ControllerInputVisualizer/Inputs/IA_Visu_FaceButton_Left.IA_Visu_FaceButton_Left"))
  ;[0 0 0 0.33 75] ControllerVisualizer Debug
  ;;[1 0.5477 0.8376 0.33] Face Button
  (:`Started`
    (`/Game/UI/Debug/ControllerInputVisualizer/WBP_ControllerInputsVisualizer.ReceiveInputVisualizationData_Button` (`self.Controller Input Visualizer`) true "NewEnumerator5"))
  (:`Completed`
    (`/Game/UI/Debug/ControllerInputVisualizer/WBP_ControllerInputsVisualizer.ReceiveInputVisualizationData_Button` (`self.Controller Input Visualizer`) false "NewEnumerator5")))

(event `EnhancedInput|/Game/_GameManager/Inputs/Actions/IA_Look`
  (params (ActionValue :type "Vector2D Structure") (ElapsedSeconds :type "Float (double-precision)") (TriggeredSeconds :type "Float (double-precision)") (InputAction :type "InputAction Object Reference" :default "/Game/_GameManager/Inputs/Actions/IA_Look.IA_Look"))
  (bind (_returnvalue_roll _returnvalue_pitch) (`KismetMathLibrary.BreakRotator` (`self.GetControlRotation`)))
  (bind (_camerafeel_fovbase _camerafeel_fovtarget _camerafeel_binvertcam _camerafeel_horizontalcamspeed _camerafeel_verticalcamspeed) (break `UCameraFeel` (`self.CameraFeel`)))
  ;[0 0 0 0.4 75] IA Look
  (:`Triggered`
    (`|ExecutionSequence`
      (:`then_0`
        (if (and (not (`self.TargetLocked`)) (`self.canPlayerMove`))
          (bind _playercharacterref (`self.PlayerCharacterRef`)
            (:`then`
              (`|ExecutionSequence`
                (:`then_0`
                  (if (not (`self.is 180 Rotating`))
                    (`Pawn.AddControllerYawInput` _playercharacterref (* ActionValue_X _camerafeel_horizontalcamspeed))
                    (`Pawn.AddControllerPitchInput` _playercharacterref (* ActionValue_Y _camerafeel_verticalcamspeed))))
                (:`then_2`
                  (`SceneComponent.K2_SetRelativeRotation` (`PlayerCharacter_Base.FirstPersonCameraComponent` _playercharacterref) (`KismetMathLibrary.MakeRotator` 0.0 _returnvalue_pitch) false false))))
            (:`else`))))
      (:`then_1`
        (if (> (`KismetMathLibrary.Abs` ActionValue_X) 0.0)
          (set `self.Last Input Yaw` ActionValue_X))))))

(event `EnhancedInput|/Game/UI/Debug/ControllerInputVisualizer/Inputs/IA_Visu_DPad_Right`
  (params (ActionValue :type Boolean) (ElapsedSeconds :type "Float (double-precision)") (TriggeredSeconds :type "Float (double-precision)") (InputAction :type "InputAction Object Reference" :default "/Game/UI/Debug/ControllerInputVisualizer/Inputs/IA_Visu_DPad_Right.IA_Visu_DPad_Right"))
  ;[0 0 0 0.33 75] ControllerVisualizer Debug
  ;;[0.3557 1 0.4036 0.33] DPad
  (:`Started`
    (`/Game/UI/Debug/ControllerInputVisualizer/WBP_ControllerInputsVisualizer.ReceiveInputVisualizationData_Button` (`self.Controller Input Visualizer`) true "NewEnumerator2"))
  (:`Completed`
    (`/Game/UI/Debug/ControllerInputVisualizer/WBP_ControllerInputsVisualizer.ReceiveInputVisualizationData_Button` (`self.Controller Input Visualizer`) false "NewEnumerator2")))

(event `EnhancedInput|/Game/UI/Debug/ControllerInputVisualizer/Inputs/IA_Visu_DPad_Top`
  (params (ActionValue :type Boolean) (ElapsedSeconds :type "Float (double-precision)") (TriggeredSeconds :type "Float (double-precision)") (InputAction :type "InputAction Object Reference" :default "/Game/UI/Debug/ControllerInputVisualizer/Inputs/IA_Visu_DPad_Top.IA_Visu_DPad_Top"))
  ;[0 0 0 0.33 75] ControllerVisualizer Debug
  ;;[0.3557 1 0.4036 0.33] DPad
  (:`Started`
    (`/Game/UI/Debug/ControllerInputVisualizer/WBP_ControllerInputsVisualizer.ReceiveInputVisualizationData_Button` (`self.Controller Input Visualizer`) true "NewEnumerator3"))
  (:`Completed`
    (`/Game/UI/Debug/ControllerInputVisualizer/WBP_ControllerInputsVisualizer.ReceiveInputVisualizationData_Button` (`self.Controller Input Visualizer`) false "NewEnumerator3")))

(event `EnhancedInput|/Game/UI/Debug/ControllerInputVisualizer/Inputs/IA_Visu_FaceButton_Top`
  (params (ActionValue :type Boolean) (ElapsedSeconds :type "Float (double-precision)") (TriggeredSeconds :type "Float (double-precision)") (InputAction :type "InputAction Object Reference" :default "/Game/UI/Debug/ControllerInputVisualizer/Inputs/IA_Visu_FaceButton_Top.IA_Visu_FaceButton_Top"))
  ;[0 0 0 0.33 75] ControllerVisualizer Debug
  ;;[1 0.5477 0.8376 0.33] Face Button
  (:`Started`
    (`/Game/UI/Debug/ControllerInputVisualizer/WBP_ControllerInputsVisualizer.ReceiveInputVisualizationData_Button` (`self.Controller Input Visualizer`) true "NewEnumerator7"))
  (:`Completed`
    (`/Game/UI/Debug/ControllerInputVisualizer/WBP_ControllerInputsVisualizer.ReceiveInputVisualizationData_Button` (`self.Controller Input Visualizer`) false "NewEnumerator7")))

(event `EnhancedInput|/Game/UI/Debug/ControllerInputVisualizer/Inputs/IA_Visu_FaceButton_Right`
  (params (ActionValue :type Boolean) (ElapsedSeconds :type "Float (double-precision)") (TriggeredSeconds :type "Float (double-precision)") (InputAction :type "InputAction Object Reference" :default "/Game/UI/Debug/ControllerInputVisualizer/Inputs/IA_Visu_FaceButton_Right.IA_Visu_FaceButton_Right"))
  ;[0 0 0 0.33 75] ControllerVisualizer Debug
  ;;[1 0.5477 0.8376 0.33] Face Button
  (:`Started`
    (`/Game/UI/Debug/ControllerInputVisualizer/WBP_ControllerInputsVisualizer.ReceiveInputVisualizationData_Button` (`self.Controller Input Visualizer`) true "NewEnumerator6"))
  (:`Completed`
    (`/Game/UI/Debug/ControllerInputVisualizer/WBP_ControllerInputsVisualizer.ReceiveInputVisualizationData_Button` (`self.Controller Input Visualizer`) false "NewEnumerator6")))

(event `EnhancedInput|/Game/UI/Debug/ControllerInputVisualizer/Inputs/IA_Visu_Shoulder_Right`
  (params (ActionValue :type Boolean) (ElapsedSeconds :type "Float (double-precision)") (TriggeredSeconds :type "Float (double-precision)") (InputAction :type "InputAction Object Reference" :default "/Game/UI/Debug/ControllerInputVisualizer/Inputs/IA_Visu_Shoulder_Right.IA_Visu_Shoulder_Right"))
  ;[0 0 0 0.33 75] ControllerVisualizer Debug
  ;;[0.9995 1 0.2907 0.33] Shoulder Buttons
  (:`Started`
    (`/Game/UI/Debug/ControllerInputVisualizer/WBP_ControllerInputsVisualizer.ReceiveInputVisualizationData_Button` (`self.Controller Input Visualizer`) true "NewEnumerator9"))
  (:`Completed`
    (`/Game/UI/Debug/ControllerInputVisualizer/WBP_ControllerInputsVisualizer.ReceiveInputVisualizationData_Button` (`self.Controller Input Visualizer`) false "NewEnumerator9")))

(event `EnhancedInput|/Game/UI/Debug/ControllerInputVisualizer/Inputs/IA_Visu_Special_Left`
  (params (ActionValue :type Boolean) (ElapsedSeconds :type "Float (double-precision)") (TriggeredSeconds :type "Float (double-precision)") (InputAction :type "InputAction Object Reference" :default "/Game/UI/Debug/ControllerInputVisualizer/Inputs/IA_Visu_Special_Left.IA_Visu_Special_Left"))
  ;[0 0 0 0.33 75] ControllerVisualizer Debug
  ;;[0.6146 0.6146 0.6146 0.33] Special Buttons
  (:`Started`
    (`/Game/UI/Debug/ControllerInputVisualizer/WBP_ControllerInputsVisualizer.ReceiveInputVisualizationData_Button` (`self.Controller Input Visualizer`) true "NewEnumerator10"))
  (:`Completed`
    (`/Game/UI/Debug/ControllerInputVisualizer/WBP_ControllerInputsVisualizer.ReceiveInputVisualizationData_Button` (`self.Controller Input Visualizer`) false "NewEnumerator10")))

(event `EnhancedInput|/Game/UI/Debug/ControllerInputVisualizer/Inputs/IA_Visu_Special_Right`
  (params (ActionValue :type Boolean) (ElapsedSeconds :type "Float (double-precision)") (TriggeredSeconds :type "Float (double-precision)") (InputAction :type "InputAction Object Reference" :default "/Game/UI/Debug/ControllerInputVisualizer/Inputs/IA_Visu_Special_Right.IA_Visu_Special_Right"))
  ;[0 0 0 0.33 75] ControllerVisualizer Debug
  ;;[0.6146 0.6146 0.6146 0.33] Special Buttons
  (:`Started`
    (`/Game/UI/Debug/ControllerInputVisualizer/WBP_ControllerInputsVisualizer.ReceiveInputVisualizationData_Button` (`self.Controller Input Visualizer`) true "NewEnumerator11"))
  (:`Completed`
    (`/Game/UI/Debug/ControllerInputVisualizer/WBP_ControllerInputsVisualizer.ReceiveInputVisualizationData_Button` (`self.Controller Input Visualizer`) false "NewEnumerator11")))

(event `EnhancedInput|/Game/UI/Debug/ControllerInputVisualizer/Inputs/IA_Visu_Shoulder_Left`
  (params (ActionValue :type Boolean) (ElapsedSeconds :type "Float (double-precision)") (TriggeredSeconds :type "Float (double-precision)") (InputAction :type "InputAction Object Reference" :default "/Game/UI/Debug/ControllerInputVisualizer/Inputs/IA_Visu_Shoulder_Left.IA_Visu_Shoulder_Left"))
  ;[0 0 0 0.33 75] ControllerVisualizer Debug
  ;;[0.9995 1 0.2907 0.33] Shoulder Buttons
  (:`Started`
    (`/Game/UI/Debug/ControllerInputVisualizer/WBP_ControllerInputsVisualizer.ReceiveInputVisualizationData_Button` (`self.Controller Input Visualizer`) true "NewEnumerator8"))
  (:`Completed`
    (`/Game/UI/Debug/ControllerInputVisualizer/WBP_ControllerInputsVisualizer.ReceiveInputVisualizationData_Button` (`self.Controller Input Visualizer`) false "NewEnumerator8")))

(event `EnhancedInput|/Game/_GameManager/Inputs/Actions/IA_LockSwitch`
  (params (ActionValue :type "Float (double-precision)") (ElapsedSeconds :type "Float (double-precision)") (TriggeredSeconds :type "Float (double-precision)") (InputAction :type "InputAction Object Reference" :default "/Game/_GameManager/Inputs/Actions/IA_LockSwitch.IA_LockSwitch"))
  (bind (_returnvalue_roll _returnvalue_pitch _returnvalue_yaw) (`KismetMathLibrary.BreakRotator` (`self.GetControlRotation`)))
  (bind _playercharacterref (`self.PlayerCharacterRef`))
  (bind _lockon_switch (`self.LockOn Switch`))
  (bind _firstpersoncameracomponent (`PlayerCharacter_Base.FirstPersonCameraComponent` _playercharacterref))
  (bind ((`TargetLockLength` _targetlocklength) (`TargetLockRadius` _targetlockradius)) (break `UPlayerFeel` (`PlayerCharacter_Base.PlayerFeel` _playercharacterref)))
  (bind (_returnvalue_roll_2 _returnvalue_pitch_2 _returnvalue_yaw_2) (`KismetMathLibrary.BreakRotator` (`SceneComponent.K2_GetComponentRotation` _firstpersoncameracomponent)))
  (bind _returnvalue (`SceneComponent.K2_GetComponentLocation` _firstpersoncameracomponent))
  ;[0 0 0 0.4 75] Lock On
  ;;[0.9 0.8 0 1 50] Target Lock On
  (:`Triggered`
    (bind _output_get (set `self.Temp Switch Action Value` ActionValue))
    (if (`self.TargetLocked`)
      (`self.SetControlRotation` (`KismetMathLibrary.MakeRotator` _returnvalue_roll _returnvalue_pitch (+ _returnvalue_yaw (* _output_get (`/Game/Characters/Player/Blueprints/BP_Player.Camera_Horizontal_Speed` (`self.As BP Player`))))))))
  (:`Started`
    (set `self.LockOn Switch` true)
    (if (`self.TargetLocked`) :!label _label_4
      (if _lockon_switch
        (bind (_outhit _returnvalue_2) (`KismetSystemLibrary.SphereTraceSingleForObjects` _returnvalue (+ _returnvalue (* (`KismetMathLibrary.GetForwardVector` (`KismetMathLibrary.MakeRotator` _returnvalue_roll_2 _returnvalue_pitch_2 (`KismetMathLibrary.SelectFloat` _returnvalue_yaw_2 (+ _returnvalue_yaw_2 (* (`KismetMathLibrary.SignOfFloat` (`self.Temp Switch Action Value`)) (`self.Angle LockOn Switch`))) (not (`self.LockOn Switch`))))) _targetlocklength)) _targetlockradius (`|MakeArray` "ObjectTypeQuery3" :!type "EObjectTypeQuery Enum") false (`|MakeArray` (`self.PlayerCharacterRef`) :!type "Actor Object Reference") "ForDuration" true (struct :`R` 1.0 :`A` 1.0) (struct :`G` 1.0 :`A` 1.0) 1.5 :!label _label_5))
        (if _returnvalue_2
          (bind (_bblockinghit _binitialoverlap _time _distance _location _impactpoint _normal _impactnormal _physmat _hitactor) (`GameplayStatics.BreakHitResult` _outhit))
          (if (`self.ActorHasTag` _hitactor "CanLockOn")
            (if (`self.ActorHasTag` _hitactor (`self.Tag Death`))
              (set `self.Lock Target Actor` null :!label _label_6)
              (set `self.TargetLocked` false)
              (else
                (set `self.Lock Target Actor` _hitactor)
                (set `self.TargetLocked` true)
                (set `self.LockOn Switch` false)))
            (elif (not (`self.LockOn Switch`))
              (goto _label_6)))
          (elif (not (`self.LockOn Switch`))
            (set `self.TargetLocked` false)))
        (else
          (set `self.Lock Target Actor` null)
          (set `self.TargetLocked` false)))
      (elif _lockon_switch
        (set `self.LockOn Switch` false)
        (else
          (goto _label_5))))))

(event `EnhancedInput|/Game/_GameManager/Inputs/Actions/IA_LockOn`
  (params (ActionValue :type Boolean) (ElapsedSeconds :type "Float (double-precision)") (TriggeredSeconds :type "Float (double-precision)") (InputAction :type "InputAction Object Reference" :default "/Game/_GameManager/Inputs/Actions/IA_LockOn.IA_LockOn"))
  ;[0 0 0 0.4 75] Lock On
  ;;[0.9 0.8 0 1 50] Target Lock On
  (:`Started`
    (set `self.LockOn Switch` false)
    (goto _label_4)))

(event `EnhancedInput|/Game/UI/Debug/ControllerInputVisualizer/Inputs/IA_Visu_StickLeft_Press`
  (params (ActionValue :type Boolean) (ElapsedSeconds :type "Float (double-precision)") (TriggeredSeconds :type "Float (double-precision)") (InputAction :type "InputAction Object Reference" :default "/Game/UI/Debug/ControllerInputVisualizer/Inputs/IA_Visu_StickLeft_Press.IA_Visu_StickLeft_Press"))
  ;[0 0 0 0.33 75] ControllerVisualizer Debug
  ;;[0.1729 0.2596 1 0.33] Stick Presses
  (:`Started`
    (`/Game/UI/Debug/ControllerInputVisualizer/WBP_ControllerInputsVisualizer.ReceiveInputVisualizationData_Button` (`self.Controller Input Visualizer`) true "NewEnumerator12"))
  (:`Completed`
    (`/Game/UI/Debug/ControllerInputVisualizer/WBP_ControllerInputsVisualizer.ReceiveInputVisualizationData_Button` (`self.Controller Input Visualizer`) false "NewEnumerator12")))

(event `SendControllerVisualizerData`
  (bind _returnvalue (subsystem `EnhancedInputLocalPlayerSubsystem`))
  ;[0 0 0 0.33 75] ControllerVisualizer Debug
  ;;[0.08067 0.6955 1 0.33] Stick Movement & Trigger Axes
  (`/Engine/EditorBlueprintResources/StandardMacros.IsValid` _returnvalue
    (:`Is Valid`
      (if (`.ReturnValue` (`EnhancedInputSubsystemInterface.HasMappingContext` _returnvalue "/Game/UI/Debug/ControllerInputVisualizer/Inputs/IMC_ControllerVisualizer.IMC_ControllerVisualizer"))
        (bind _controller_input_visualizer (`self.Controller Input Visualizer`)
          (:`then`
            (`/Game/UI/Debug/ControllerInputVisualizer/WBP_ControllerInputsVisualizer.ReceiveInputVisualizationData_Stick` _controller_input_visualizer (`|GetInputActionValue`) true)
            (`/Game/UI/Debug/ControllerInputVisualizer/WBP_ControllerInputsVisualizer.ReceiveInputVisualizationData_Stick` (`self.Controller Input Visualizer`) (`|GetInputActionValue`) false)
            (`/Game/UI/Debug/ControllerInputVisualizer/WBP_ControllerInputsVisualizer.ReceiveInputVisualizationData_Axis` (`self.Controller Input Visualizer`) (`|GetInputActionValue`) true)
            (`/Game/UI/Debug/ControllerInputVisualizer/WBP_ControllerInputsVisualizer.ReceiveInputVisualizationData_Axis` (`self.Controller Input Visualizer`) (`|GetInputActionValue`) false))
          (:`else`))))))

(event `EnhancedInput|/Game/UI/Debug/ControllerInputVisualizer/Inputs/IA_Visu_StickRight_Press`
  (params (ActionValue :type Boolean) (ElapsedSeconds :type "Float (double-precision)") (TriggeredSeconds :type "Float (double-precision)") (InputAction :type "InputAction Object Reference" :default "/Game/UI/Debug/ControllerInputVisualizer/Inputs/IA_Visu_StickRight_Press.IA_Visu_StickRight_Press"))
  ;[0 0 0 0.33 75] ControllerVisualizer Debug
  ;;[0.1729 0.2596 1 0.33] Stick Presses
  (:`Started`
    (`/Game/UI/Debug/ControllerInputVisualizer/WBP_ControllerInputsVisualizer.ReceiveInputVisualizationData_Button` (`self.Controller Input Visualizer`) true "NewEnumerator13"))
  (:`Completed`
    (`/Game/UI/Debug/ControllerInputVisualizer/WBP_ControllerInputsVisualizer.ReceiveInputVisualizationData_Button` (`self.Controller Input Visualizer`) false "NewEnumerator13")))

(event `EnhancedInput|/Game/_GameManager/Inputs/Actions/IA_180`
  (params (ActionValue :type Boolean) (ElapsedSeconds :type "Float (double-precision)") (TriggeredSeconds :type "Float (double-precision)") (InputAction :type "InputAction Object Reference" :default "/Game/_GameManager/Inputs/Actions/IA_180.IA_180"))
  (bind (_returnvalue_roll _returnvalue_pitch _returnvalue_yaw) (`KismetMathLibrary.BreakRotator` (`self.GetControlRotation`)))
  ;[0 0 0 0.4 75] 180 Rotation
  ;;[0.2 1 0.2 1 50] 180 Rotation
  (:`Triggered`
    (if (and (`self.canPlayerMove`) (not (`self.is 180 Rotating`)))
      (set `self.is 180 Rotating` true)
      (`MovementComponent.StopMovementImmediately` (`Character.CharacterMovement` (`self.PlayerCharacterRef`)))
      (set `self.Lock Target Actor` null)
      (set `self.TargetLocked` false)
      (bind _output_get (set `self.Temp Rotation` (`KismetMathLibrary.MakeRotator` _returnvalue_roll _returnvalue_pitch (+ _returnvalue_yaw (* (`self.180_Rotation`) (`KismetMathLibrary.SignOfFloat` (`self.Last Input Yaw`)))))))
      (bind (_direction _rotation_speed) (`Timeline|T_Rotation` :!via `PlayFromStart`)
        (:`Update`
          _)
        (:`Finished`
          (set `self.is 180 Rotating` false)))
      (`self.SetControlRotation` (`KismetMathLibrary.RLerp` (`self.GetControlRotation`) _output_get _rotation_speed)))))

(event `CustomEvent`
  (params (Visibility :type Boolean))
  ;[0 0 0 0.33 75] ControllerVisualizer Debug
  (`/Game/UI/Debug/ControllerInputVisualizer/WBP_ControllerInputsVisualizer.SetUIVisibility` (`self.Controller Input Visualizer`) Visibility))

(fn `Generate Widget`
  (bind _returnvalue (`|CreateWidget` "/Game/UI/Menus/InGameMenu/WBP_InGameMenu.WBP_InGameMenu_C"))
  (bind _output_get (set `self.WBP InGameMenu` _returnvalue))
  (`UserWidget.AddToViewport` _output_get 0)
  (set `self.StunWidget` (`/Game/UI/Menus/InGameMenu/WBP_InGameMenu.WBP_Stun` _returnvalue))
  (set `self.Controller Input Visualizer` (`/Game/UI/Menus/InGameMenu/WBP_InGameMenu.WBP_ControllerInputsVisualizer` _returnvalue))
  (set `self.WBP Healing Effect` (`/Game/UI/Menus/InGameMenu/WBP_InGameMenu.WBP_HealingEffect` _returnvalue))
  (set `self.WBP Damage Effect` (`/Game/UI/Menus/InGameMenu/WBP_InGameMenu.WBP_DamagePurcentEffect` _returnvalue))
  (set `self.WBP Hurt Screen Effect` (`/Game/UI/Menus/InGameMenu/WBP_InGameMenu.WBP_HurtScreenEffect` _returnvalue))
  (set `self.WBP Death Screen` (`/Game/UI/Menus/InGameMenu/WBP_InGameMenu.WBP_DeathScreen` _returnvalue))
  (set `self.WBp Loading Screen` (`/Game/UI/Menus/InGameMenu/WBP_InGameMenu.WBp_LoadingScreen` _returnvalue))
  (set `self.WBP Scoring` (`/Game/UI/Menus/InGameMenu/WBP_InGameMenu.WBP_Scoring` _returnvalue))
  (set `self.WBP End Screen` (`/Game/UI/Menus/InGameMenu/WBP_InGameMenu.WBP_EndScreen` _returnvalue))
  (set `self.WBP One Minute Left` (`/Game/UI/Menus/InGameMenu/WBP_InGameMenu.WBP_OneMinuteLeft` _returnvalue))
  (set `self.WBP Big Number` (`/Game/UI/Menus/InGameMenu/WBP_InGameMenu.WBP_BigNumber` _returnvalue))
  (set `self.WBP Dialogue Cinematic` (`/Game/UI/Menus/InGameMenu/WBP_InGameMenu.WBP_Dialogue_Cinematic` _returnvalue))
  (set `self.WBP Dialogue in Game` (`/Game/UI/Menus/InGameMenu/WBP_InGameMenu.WBP_Dialogue_In_Game` _returnvalue))
  (`Widget.SetVisibility` _returnvalue "Visible"))

(fn `SetCameraFeel`
  (bind _data_asset_player (`self.Data_Asset_Player`))
  (setmembers `UCameraFeel` :`StructRef` (`self.CameraFeel`) :`FOVBase` (`/Game/_GameManager/Data_Assets/Data_3C/PDA_Player.Current_FOV` _data_asset_player) :`FOVTarget` (`/Game/_GameManager/Data_Assets/Data_3C/PDA_Player.Dash_FOV` _data_asset_player) :`bInvertCam` (`/Game/_GameManager/Data_Assets/Data_3C/PDA_Player.Camera_Invert` _data_asset_player) :`HorizontalCamSpeed` (`/Game/_GameManager/Data_Assets/Data_3C/PDA_Player.Camera_Horizontal_Speed` _data_asset_player) :`VerticalCamSpeed` (`/Game/_GameManager/Data_Assets/Data_3C/PDA_Player.Camera_Vertical_Speed` _data_asset_player) :`ViewPitchMin` (`/Game/_GameManager/Data_Assets/Data_3C/PDA_Player.Camera_View_Pitch_Min` _data_asset_player) :`ViewPitchMax` (`/Game/_GameManager/Data_Assets/Data_3C/PDA_Player.Camera_View_Pitch_Max` _data_asset_player)))

(fn `UserConstructionScript`)