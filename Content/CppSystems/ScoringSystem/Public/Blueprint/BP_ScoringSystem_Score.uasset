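; Blueprint score component of the scoring system that adds points and multiplier percentage and shows the result on screen.
; It takes the scoring widget from the PC_Systems controller and uses that widget as world context for delays and timer clearing.
; Each increase reveals the score if hidden, updates the total and spawns an added-points popup.
; A timer restarted on each increase reverses the reveal animation after a few seconds without scoring.
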(event `self.InitializeBlueprint`
  (`parent.InitializeBlueprint`))

(event `InitWorldContext`
  (params (Controller :type "PlayerController Object Reference"))
  (bind _aspc_systems (cast `/Game/_GameManager/PC_Systems` Controller))
  (set `self.WBP Scoring` (`/Game/_GameManager/PC_Systems.WBP Scoring` _aspc_systems)))

(event `self.DeinitializeBlueprint`
  (`parent.DeinitializeBlueprint`))

(event `self.IncreaseWithText`
  (params (InScoreIncrease :type Integer) (InMultiplierPercentageIncrease :type Integer) (InMessage :type "Text (by ref)"))
  (bind _wbp_scoring (`self.WBP Scoring`))
  (bind _wbp_scoring_2 (`self.WBP Scoring`))
  (`self.WBP Scoring`
    (:`then`
      ; Score display + update
      (if (not (`self.bIsScoreIncreasing`))
        (`UserWidget.PlayAnimation` _wbp_scoring_2 (`/Game/UI/Menus/InGameMenu/WBP_Scoring.DisplayScore` _wbp_scoring_2) 0.0 1 "Forward" 1.0 false)
        (`KismetSystemLibrary.Delay` (`self.WBP Scoring`) 0.5)
        (set `self.bIsScoreIncreasing` true))
      (`KismetSystemLibrary.K2_ClearAndInvalidateTimerHandle` (`self.WBP Scoring`) (`self.ScoreTimerHandle`))
      (bind _returnvalue (`KismetSystemLibrary.K2_SetTimerDelegate` (delegate `HideScore`) 3.0))
      (set `self.ScoreTimerHandle` _returnvalue)
      (`self.Increase` InScoreIncrease InMultiplierPercentageIncrease)
      (`/Game/UI/Menus/InGameMenu/WBP_Scoring.SetTextScore` _wbp_scoring (`self.GetScore`))
      (`KismetSystemLibrary.Delay` (`self.WBP Scoring`) 0.1)
      (`/Game/UI/Menus/InGameMenu/WBP_Scoring.SpawnAddingScore` _wbp_scoring InScoreIncrease))
    (:`else`)))

(event `HideScore`
  (bind _wbp_scoring (`self.WBP Scoring`))
  ; Score display + update
  (`UserWidget.PlayAnimationReverse` _wbp_scoring (`/Game/UI/Menus/InGameMenu/WBP_Scoring.DisplayScore` _wbp_scoring) 1.0 false)
  (`KismetSystemLibrary.Delay` (`self.WBP Scoring`) 0.5)
  (set `self.bIsScoreIncreasing` false))