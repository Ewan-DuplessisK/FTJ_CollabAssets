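; Scoring actor component that raises the score and multiplier percentage and reflects the change in the scoring UI.
; On BeginPlay it caches the WBPScoring widget from the first player controller, cast to PC_Systems.
; IncreasewithText calls Increase, sets the score text from GetScore, then after a short delay spawns the added-score display on the widget.
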(event `self.ReceiveBeginPlay`
  (bind _aspc_systems (cast `/Game/_GameManager/PC_Systems` (`GameplayStatics.GetPlayerController` 0)))
  (set `self.WBP Scoring` (`/Game/_GameManager/PC_Systems.WBP Scoring` _aspc_systems)))

(event `self.IncreaseWithText`
  (params (InScoreIncrease :type Integer) (InMultiplierPercentageIncrease :type Integer) (InMessage :type "Text (by ref)"))
  (bind _wbp_scoring (`self.WBP Scoring`))
  ; Score display + update
  (`self.Increase` InScoreIncrease InMultiplierPercentageIncrease)
  (`/Game/UI/Menus/InGameMenu/WBP_Scoring.SetTextScore` _wbp_scoring (`self.GetScore`))
  (`KismetSystemLibrary.Delay` 0.1)
  (`/Game/UI/Menus/InGameMenu/WBP_Scoring.SpawnAddingScore` _wbp_scoring InScoreIncrease))