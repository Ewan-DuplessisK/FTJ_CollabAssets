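; Breakable office security camera that rotates its mesh every tick to face the player character until broken.
; An overlap on its box by an actor tagged Heavy, Medium or Light breaks it once, hiding the meshes and disabling their collision.
; Breaking also adds "Broke Cam" score and multiplier through the player's scoring component.
; An OnHit dispatcher, bound at BeginPlay, triggers the hit sound and Niagara break effects.
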(event `self.ReceiveBeginPlay`
  (`self.Init Feedback`))

(event `self.ReceiveTick`
  (params (DeltaSeconds :type "Float (single-precision)"))
  (bind _sm_camera (`self.SM_Camera`))
  (bind (_returnvalue_roll _returnvalue_pitch _returnvalue_yaw) (`KismetMathLibrary.BreakRotator` (`KismetMathLibrary.FindLookAtRotation` (`SceneComponent.K2_GetComponentLocation` _sm_camera) (`self.K2_GetActorLocation` (`GameplayStatics.GetPlayerCharacter` 0)))))
  (if (not (`self.Is Broken`))
    (`SceneComponent.K2_SetWorldRotation` _sm_camera (`KismetMathLibrary.MakeRotator` _returnvalue_roll _returnvalue_pitch _returnvalue_yaw) false false)))

(event `self.Box.OnComponentBeginOverlap`
  (params (OverlappedComponent :type "PrimitiveComponent Object Reference") (OtherActor :type "Actor Object Reference") (OtherComp :type "PrimitiveComponent Object Reference") (OtherBodyIndex :type Integer) (bFromSweep :type Boolean) (SweepResult :type "HitResult Structure (by ref)"))
  (if (or (`self.ActorHasTag` OtherActor "Heavy") (`self.ActorHasTag` OtherActor "Medium") (`self.ActorHasTag` OtherActor "Light"))
    (if (not (`self.Is Broken`))
      (set `self.Is Broken` true)
      (`self.On Hit`)
      (for _array_element (`|MakeArray` (`self.SM_Wall_Fixture`) (`self.SM_Camera`) (`self.SM_Rotating_Nub`))
        (`SceneComponent.SetVisibility` _array_element false false)
        (`PrimitiveComponent.SetCollisionEnabled` _array_element "NoCollision"))
      (`FTJ_ScoringSystem_Score.IncreaseWithText` (`self.GetComponentByClass` (`GameplayStatics.GetPlayerCharacter` 0) "/Game/CppSystems/ScoringSystem/Public/ActorComponent/BP_ScoringSystem_Score_AC.BP_ScoringSystem_Score_AC_C") 5 1 (`|FormatText` "Broke Cam")))))

(event `Init Feedback`
  (`|ExecutionSequence`
    (:`then_0`
      (add `self.On Hit` (delegate `On Hit_Event`)))))

(event `On Hit_Event`
  (bind _sm_camera (`self.SM_Camera`))
  (bind _returnvalue (`SceneComponent.K2_GetComponentLocation` _sm_camera))
  (bind _returnvalue_2 (`SceneComponent.K2_GetComponentRotation` _sm_camera))
  (bind _returnvalue_3 (/ (`self.GetActorScale3D`) 12.0))
  ;[0 1 1 0.5] Sound When Hit
  (`GameplayStatics.SpawnSoundAtLocation` (`self.Sound When Hit`) (0.0 0.0 0.0) (struct) 1.0 1.0 0.0 null null)
  ;[0 1 1] VFX
  (`NiagaraFunctionLibrary.SpawnSystemAtLocation` (`self.VFX When Hit`) _returnvalue _returnvalue_2 _returnvalue_3)
  (`NiagaraFunctionLibrary.SpawnSystemAtLocation` "/Game/VFX/Niagara/Props/NS_Machine_Break.NS_Machine_Break" _returnvalue _returnvalue_2 _returnvalue_3))

(fn `UserConstructionScript`)